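; Player controller that relays axis and Select input to the controlled pawn.
; On BeginPlay it caches a pawn reference through GetPlayerMessage, shows the mouse cursor and enables HZB occlusion by console command.
; Vertical and Horizontal axes pass a small dead zone before calling the pawn's move functions, while Select press and release call Select and EndSelect, all guarded by validity checks.
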(event `self.ReceiveBeginPlay`
  (bind _playerref (message `/Game/Blueprints/Player/BPI_Player.GetPlayer` (`self.K2_GetPawn`)))
  (set `self.Player Ref` _playerref)
  (set `self.bShowMouseCursor` true)
  (`KismetSystemLibrary.ExecuteConsoleCommand` "r.HZBOcclusion 1" null))

(event `InputAxis|Vertical`
  (params (AxisValue :type "Float (single-precision)"))
  (bind _player_ref (`self.Player Ref`))
  (if (or (> AxisValue 0.1) (< AxisValue -0.1))
    (`/Engine/EditorBlueprintResources/StandardMacros.IsValid` _player_ref
      (:`Is Valid`
        (`/Game/Blueprints/Player/BP_PlayerPawn.MoveVertical` _player_ref AxisValue)))))

(event `InputAxis|Horizontal`
  (params (AxisValue :type "Float (single-precision)"))
  (bind _player_ref (`self.Player Ref`))
  (if (or (> AxisValue 0.1) (< AxisValue -0.1))
    (`/Engine/EditorBlueprintResources/StandardMacros.IsValid` _player_ref
      (:`Is Valid`
        (`/Game/Blueprints/Player/BP_PlayerPawn.MoveHorizontal` _player_ref AxisValue)))))

(event `InputAction|Select`
  (params (Key :type "Key Structure"))
  (bind _player_ref (`self.Player Ref`))
  (:`Pressed`
    (`/Engine/EditorBlueprintResources/StandardMacros.IsValid` _player_ref
      (:`Is Valid`
        (`/Game/Blueprints/Player/BP_PlayerPawn.Select` _player_ref))))
  (:`Released`
    (`/Engine/EditorBlueprintResources/StandardMacros.IsValid` _player_ref
      (:`Is Valid`
        (`/Game/Blueprints/Player/BP_PlayerPawn.EndSelect` _player_ref)))))

(fn `UserConstructionScript`)