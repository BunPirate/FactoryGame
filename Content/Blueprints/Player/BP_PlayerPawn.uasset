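; Player pawn for a tile-based building game, providing a panning, zooming camera and Select, Place and Destroy mouse modes.
; Cursor traces become tile coordinates, and BP_TileManager handles placing and removing buildings.
; Drags run looping timers that preview straight rows or destroy areas, committed on release, while multi-tile buildings place on click with rotatable, validity-colored previews.
; Mode changes clear previews and update the HUD and cursor widget.
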(event `self.ReceiveBeginPlay`
  ;[1 1 1] Pawn Init
  (bind _returnvalue (`GameplayStatics.GetActorOfClass` "/Game/Blueprints/BP_TileManager.BP_TileManager_C"))
  (set `self.TileManagerRef` _returnvalue)
  (bind _returnvalue_2 (`GameplayStatics.GetActorOfClass` "/Game/Blueprints/BP_LevelGenerator.BP_LevelGenerator_C"))
  (set `self.LevelGeneratorRef` _returnvalue_2)
  (bind _asbp_player_controller (cast `/Game/Blueprints/Player/BP_PlayerController` (`GameplayStatics.GetPlayerController` 0)))
  (set `self.PlayerController` _asbp_player_controller))

(event `self.ReceiveTick`
  (params (DeltaSeconds :type "Float (single-precision)"))
  (bind (_lastmousecoordinate_x _lastmousecoordinate_y) (break `/Game/Blueprints/Structures/IntVector2` (`self.LastMouseCoordinate`)))
  (bind _cursorwidget (`/Game/Blueprints/Player/BP_PlayerController.CursorWidget` (`self.PlayerController`)))
  ;[1 1 1] Update Camera Position
  (`SceneComponent.K2_SetWorldTransform` (`self.DefaultSceneRoot`) (`KismetMathLibrary.MakeTransform` (`self.CamLocation`) (`self.CamRotation`)) false false)
  (switch `/Game/Blueprints/Enums/E_PlayerMode` (`self.CurrentMode`)
    (:`NewEnumerator0`
      (bind _tileref (message `/Game/Blueprints/Interfaces/BPI_Tile.GetTile` (`.HitActor` (`GameplayStatics.BreakHitResult` (`PlayerController.GetHitResultUnderCursorForObjects` (`self.PlayerController`) (`|MakeArray` "ObjectTypeQuery8" :!type "EObjectTypeQuery Enum") true)))))
      (`/Engine/EditorBlueprintResources/StandardMacros.IsValid` _tileref
        (:`Is Valid`
          (if (`/Game/Blueprints/Tiles/BP_TileBase.PlayerInteractable` _tileref)
            (`/Game/Blueprints/UI/W_Cursor.SwapCursor` _cursorwidget "NewEnumerator1")
            (else
              (`/Game/Blueprints/UI/W_Cursor.SwapCursor` _cursorwidget "NewEnumerator0" :!label _label))))
        (:`Is Not Valid`
          (goto _label))))
    (:`NewEnumerator1`
      ;[1 1 1] Building tile preview
      (bind (_isempty_ _coordinate) (`self.GetTileUnderMouse`))
      (bind (_x _y) (break `/Game/Blueprints/Structures/IntVector2` _coordinate))
      (if (not (and (== _lastmousecoordinate_x _x) (== _lastmousecoordinate_y _y)))
        (set `self.LastMouseCoordinate` _coordinate)
        (`self.SpawnMultibuildingPreview`)
        (`/Game/Blueprints/UI/W_Cursor.SwapCursor` (`/Game/Blueprints/Player/BP_PlayerController.CursorWidget` (`self.PlayerController`)) "NewEnumerator3")))))

(event `MoveVertical`
  (params (Axis :type "Float (double-precision)"))
  ;[1 1 1] Move Vertical Axis
  (set `self.CamLocation` (`KismetMathLibrary.MakeVector` (+ (* Axis (`GameplayStatics.GetWorldDeltaSeconds`) (`self.CamSpeed`) (`KismetMathLibrary.MapRangeClamped` (`self.ZoomAlpha`) 0.0 1.0 1.0 0.25)) (.x (`self.CamLocation`))) (.y (`self.CamLocation`)) (.z (`self.CamLocation`)))))

(event `ForceUpdatePreview`
  ;[1 1 1] Building tile preview
  (bind (_isempty_ _coordinate) (`self.GetTileUnderMouse`))
  (set `self.LastMouseCoordinate` _coordinate)
  (`self.SpawnMultibuildingPreview`))

(event `MoveHorizontal`
  (params (Axis :type "Float (double-precision)"))
  ;[1 1 1] Move Horizontal Axis
  (set `self.CamLocation` (`KismetMathLibrary.MakeVector` (.x (`self.CamLocation`)) (+ (* Axis (`GameplayStatics.GetWorldDeltaSeconds`) (`self.CamSpeed`) (`KismetMathLibrary.MapRangeClamped` (`self.ZoomAlpha`) 0.0 1.0 1.0 0.25)) (.y (`self.CamLocation`))) (.z (`self.CamLocation`)))))

(event `InputAxis|Zoom`
  (params (AxisValue :type "Float (single-precision)"))
  (bind _springarm (`self.SpringArm`))
  (bind _zoomalpha (`self.ZoomAlpha`))
  ;[1 1 1] Zoom in camera
  (bind _output_get (set `self.ZoomAlpha` (`KismetMathLibrary.FClamp` (+ (* AxisValue (`self.ZoomSpeed`) (`GameplayStatics.GetWorldDeltaSeconds`)) (`self.ZoomAlpha`)))))
  (`SceneComponent.K2_SetRelativeLocation` (`self.SpringArm`) (`KismetMathLibrary.MakeVector` (`KismetMathLibrary.Lerp` -5000.0 -100.0 _output_get) (.y (`SceneComponent.RelativeLocation` (`self.SpringArm`))) (.z (`SceneComponent.RelativeLocation` (`self.SpringArm`)))) false false)
  (if (> _zoomalpha 0.75)
    (`SceneComponent.K2_SetRelativeRotation` _springarm (`KismetMathLibrary.RLerp` (struct) (struct :`Pitch` 25.0) (`KismetMathLibrary.MapRangeClamped` _zoomalpha 0.75 1.0 0.0 1.0)) false false)
    (else
      (`SceneComponent.K2_SetRelativeRotation` :`self` _springarm))))

(event `DestroyAreaPreview`
  ;[1 1 1] Preview tick
  (bind (_isempty_ _coordinate) (`self.GetTileUnderMouse`))
  (set `self.SelectionEndPos` _coordinate)
  (`self.SpawnDestroyAreaPreview` (`self.SelectionStartPos`) (`self.SelectionEndPos`)))

(event `ChangeMode`
  (params (CurrentMode :type "/Game/Blueprints/Enums/E_PlayerMode Enum" :default "NewEnumerator0"))
  (bind _playercontroller (`self.PlayerController`))
  (bind _cursorwidget (`/Game/Blueprints/Player/BP_PlayerController.CursorWidget` _playercontroller))
  (bind _hudref (`/Game/Blueprints/Player/BP_PlayerController.HudRef` _playercontroller))
  ;[1 1 1] Changes the current mouse mode
  (bind _output_get (set `self.CurrentMode` CurrentMode))
  (set `self.CurrentTileClass` (struct))
  (`KismetSystemLibrary.K2_ClearAndInvalidateTimerHandle` (`self.TimerHandle`))
  (`self.ClearPreviewTiles`)
  (switch `/Game/Blueprints/Enums/E_PlayerMode` _output_get
    (:`NewEnumerator0`
      (`/Game/Blueprints/UI/W_HUD.HideRequrementsMenu` _hudref)
      (`/Game/Blueprints/UI/W_Cursor.SwapCursor` _cursorwidget "NewEnumerator0" :!label _label_2))
    (:`NewEnumerator1`
      (`/Game/Blueprints/UI/W_HUD.ShowRequrementsMenu` _hudref)
      (goto _label_2))
    (:`NewEnumerator3`
      (`/Game/Blueprints/UI/W_Cursor.SwapCursor` _cursorwidget "NewEnumerator2")
      (`/Game/Blueprints/UI/W_HUD.HideRequrementsMenu` _hudref))))

(event `RenderPreview`
  ;[1 1 1] Preview tick
  (bind (_isempty_ _coordinate) (`self.GetTileUnderMouse`))
  (`self.SpawnPreviewRow` (`self.SelectionStartPos`) _coordinate))

(event `Select`
  (bind (_currenttileclass_name _currenttileclass_icon _currenttileclass_class _currenttileclass_size _currenttileclass_multitile) (break `/Game/Blueprints/Structures/S_BuildingInfo` (`self.CurrentTileClass`)))
  ;[1 1 1] Drag start
  (bind (_isempty_ _coordinate) (`self.GetTileUnderMouse`))
  (set `self.SelectionStartPos` _coordinate)
  (`/Game/Blueprints/UI/W_Cursor.PlayClickCursor` (`/Game/Blueprints/Player/BP_PlayerController.CursorWidget` (`self.PlayerController`)))
  (switch `/Game/Blueprints/Enums/E_PlayerMode` (`self.CurrentMode`)
    (:`NewEnumerator0`
      (bind _tileref (message `/Game/Blueprints/Interfaces/BPI_Tile.GetTile` (`.HitActor` (`GameplayStatics.BreakHitResult` (`PlayerController.GetHitResultUnderCursorForObjects` (`self.PlayerController`) (`|MakeArray` "ObjectTypeQuery8" :!type "EObjectTypeQuery Enum") true)))))
      (`/Engine/EditorBlueprintResources/StandardMacros.IsValid` _tileref
        (:`Is Valid`
          (if (`/Game/Blueprints/Tiles/BP_TileBase.PlayerInteractable` _tileref)
            (message `/Game/Blueprints/Interfaces/BPI_Tile.Interact` _tileref)))))
    (:`NewEnumerator1`
      (if _currenttileclass_multitile
        (`/Game/Blueprints/BP_TileManager.PlaceMultiTileBuilding` (`self.TileManagerRef`) _coordinate (`self.Rotation`) (`self.CurrentTileClass`))
        (else
          ;[1 1 1] Preview tick
          (bind _returnvalue (`KismetSystemLibrary.K2_SetTimerDelegate` (delegate `RenderPreview`) 0.1 true))
          (set `self.TimerHandle` _returnvalue))))
    (:`NewEnumerator3`
      ;[1 1 1] Preview tick
      (bind _returnvalue_2 (`KismetSystemLibrary.K2_SetTimerDelegate` (delegate `DestroyAreaPreview`) 0.1 true))
      (set `self.DestroyAreaHandle` _returnvalue_2))))

(event `SpawnMultibuildingPreview`
  (bind _multibuildingpreviewactors (`self.MultibuildingPreviewActors`))
  ;[1 1 1] Spawns preview for creating large buildings
  (bind _values (`BlueprintMapLibrary.Map_Values` _multibuildingpreviewactors))
  (for _array_element _values
    (`/Engine/EditorBlueprintResources/StandardMacros.IsValid` _array_element
      (:`Is Valid`
        (`self.K2_DestroyActor` _array_element))))
  (`BlueprintMapLibrary.Map_Clear` _multibuildingpreviewactors)
  (bind (_isempty_ _coordinate) (`self.GetTileUnderMouse`))
  (`self.MultiTilePreview` (`self.CurrentTileClass`) _coordinate (`self.Rotation`)))

(event `SetCurrentTile`
  (params (BuildingType :type "/Game/Blueprints/Structures/S_BuildingInfo Structure"))
  ;[1 1 1] Sets current tile
  (`self.ChangeMode` "NewEnumerator1")
  (set `self.CurrentTileClass` BuildingType)
  (`/Game/Blueprints/UI/W_HUD.UpdateRequrementsSlots` (`/Game/Blueprints/Player/BP_PlayerController.HudRef` (`self.PlayerController`))))

(event `EndSelect`
  (bind _previewactors (`self.PreviewActors`))
  (bind (_currenttileclass_name _currenttileclass_icon _currenttileclass_class _currenttileclass_size _currenttileclass_multitile) (break `/Game/Blueprints/Structures/S_BuildingInfo` (`self.CurrentTileClass`)))
  ;[1 1 1] Drag end
  (bind (_isempty_ _coordinate) (`self.GetTileUnderMouse`))
  (set `self.SelectionEndPos` _coordinate)
  (switch `/Game/Blueprints/Enums/E_PlayerMode` (`self.CurrentMode`)
    (:`NewEnumerator1`
      ;[1 1 1] Place tiles
      (if _currenttileclass_multitile
        (`self.ForceUpdatePreview`)
        (else
          (`self.ForceUpdatePreview`)
          ;;[1 1 1] Spawn the actual tiles
          (`self.Place Row Of Tiles` (`self.SelectionStartPos`) (`self.SelectionEndPos`) (`self.CurrentTileClass`))
          (`KismetSystemLibrary.K2_ClearAndInvalidateTimerHandle` (`self.TimerHandle`))
          ;;[1 1 1] Clear the preview tiles
          (bind _values (`BlueprintMapLibrary.Map_Values` _previewactors))
          (for (_array_element _array_index) _values
            (`/Engine/EditorBlueprintResources/StandardMacros.IsValid` _array_element
              (:`Is Valid`
                (`/Game/Blueprints/Tiles/BP_TilePreview.RemovePreviewTile` _array_element)
                (bind _keys (`BlueprintMapLibrary.Map_Keys` _previewactors))
                (`BlueprintMapLibrary.Map_Remove` _previewactors (`|GetArrayItem` _keys _array_index))))))))
    (:`NewEnumerator3`
      ;[1 1 1] Destroy tiles
      (`InstancedStaticMeshComponent.ClearInstances` (`/Game/Blueprints/BP_TileManager.InstancedStaticMesh` (`self.TileManagerRef`)))
      (`KismetSystemLibrary.K2_ClearAndInvalidateTimerHandle` (`self.DestroyAreaHandle`))
      (`self.DestroyInArea` (`self.SelectionStartPos`) (`self.SelectionEndPos`) true)
      (`/Game/Blueprints/UI/W_Cursor.PlayWiggleCursor` (`/Game/Blueprints/Player/BP_PlayerController.CursorWidget` (`self.PlayerController`))))))

(event `Key|R`
  (params (Key :type "Key Structure"))
  ;[1 1 1] Rotate Tile
  (:`Pressed`
    (bind _output_get (set `self.RotationIndex` (+ (`self.RotationIndex`) 1)))
    (if (> _output_get 3)
      (bind _output_get_2 (set `self.RotationIndex` 0)))
    (set `self.Rotation` (select `/Game/Blueprints/Enums/E_Direction` (cast `/Game/Blueprints/Enums/E_Direction` _output_get_2) :`NewEnumerator0` "NewEnumerator0" :`NewEnumerator1` "NewEnumerator3" :`NewEnumerator2` "NewEnumerator1" :`NewEnumerator3` "NewEnumerator2" :!type "/Game/Blueprints/Enums/E_Direction Enum"))
    (`self.ForceUpdatePreview`)
    (`/Game/Blueprints/UI/W_Cursor.SetDirectionCursor` (`/Game/Blueprints/Player/BP_PlayerController.CursorWidget` (`self.PlayerController`)) (`self.Rotation`))))

(event `Key|Escape`
  (params (Key :type "Key Structure"))
  (:`Pressed`
    (`self.ChangeMode` "NewEnumerator0" :!label _label_3)))

(event `Key|RightMouseButton`
  (params (Key :type "Key Structure"))
  (:`Pressed`
    (goto _label_3)))

(event `Key|One`
  (params (Key :type "Key Structure"))
  ;[1 1 1] Debug spawn enemy
)

(event `Key|Two`
  (params (Key :type "Key Structure"))
  ;[1 1 1] Debug spawn turret
)

(fn `ClearPreviewTiles`
  (bind _multibuildingpreviewactors (`self.MultibuildingPreviewActors`))
  (bind _previewactors (`self.PreviewActors`))
  (bind _values (`BlueprintMapLibrary.Map_Values` _previewactors))
  (for _array_element _values
    (`/Engine/EditorBlueprintResources/StandardMacros.IsValid` _array_element
      (:`Is Valid`
        (`/Game/Blueprints/Tiles/BP_TilePreview.RemovePreviewTile` _array_element))))
  (`BlueprintMapLibrary.Map_Clear` _previewactors)
  (bind _values_2 (`BlueprintMapLibrary.Map_Values` _multibuildingpreviewactors))
  (for _array_element_2 _values_2
    (`/Engine/EditorBlueprintResources/StandardMacros.IsValid` _array_element_2
      (:`Is Valid`
        (`/Game/Blueprints/Tiles/BP_TilePreview.RemovePreviewTile` _array_element_2))))
  (`BlueprintMapLibrary.Map_Clear` _multibuildingpreviewactors)
  (return))

(fn `DecideTileDirection`
  (params (`Is X Greater` :type Boolean) (IsNegative :type Boolean))
  (returns (Direction :type "/Game/Blueprints/Enums/E_Direction Enum"))
  (if `Is X Greater`
    (if IsNegative
      (return "NewEnumerator0")
      (else
        (return "NewEnumerator1")))
    (elif IsNegative
      (return "NewEnumerator3")
      (else
        (return "NewEnumerator2")))))

(fn `DestroyInArea`
  (params (StartPos :type "/Game/Blueprints/Structures/IntVector2 Structure (by ref)") (EndPos :type "/Game/Blueprints/Structures/IntVector2 Structure") (`PlayerDestroyed?` :type Boolean))
  (bind (_x _y) (break `/Game/Blueprints/Structures/IntVector2` StartPos))
  (bind (_x_2 _y_2) (break `/Game/Blueprints/Structures/IntVector2` EndPos))
  (bind (_x_3 _y_3) (break `/Game/Blueprints/Structures/IntVector2` StartPos))
  (bind (_x_4 _y_4) (break `/Game/Blueprints/Structures/IntVector2` (make `/Game/Blueprints/Structures/IntVector2` (`KismetMathLibrary.Clamp` (- (`KismetMathLibrary.Abs_Int` (`KismetMathLibrary.Max` _x _x_2)) (`KismetMathLibrary.Abs_Int` (`KismetMathLibrary.Min` _x _x_2))) 0 16) (`KismetMathLibrary.Clamp` (- (`KismetMathLibrary.Abs_Int` (`KismetMathLibrary.Max` _y _y_2)) (`KismetMathLibrary.Abs_Int` (`KismetMathLibrary.Min` _y _y_2))) 0 16))))
  ;[1 1 1] X
  (for _index (range (+ _x_4 1))
    ;[1 1 1] Y
    (for _index_2 (range (+ _y_4 1))
      (`/Game/Blueprints/BP_TileManager.RemoveBuilding` (`self.TileManagerRef`) (make `/Game/Blueprints/Structures/IntVector2` (+ (* _index (select `bool` (< _x _x_2) :`false` -1 :`true` 1)) _x_3) (+ (* _index_2 (select `bool` (< _y _y_2) :`false` -1 :`true` 1)) _y_3)) `PlayerDestroyed?`)))
  (return))

(fn `GetPlayer`
  (returns (PlayerRef :type "/Game/Blueprints/Player/BP_PlayerPawn Object Reference"))
  (return self))

(fn `GetTileUnderMouse`
  (returns (`IsEmpty?` :type Boolean) (Coordinate :type "/Game/Blueprints/Structures/IntVector2 Structure") (WorldLocation :type "Vector Structure"))
  (bind (_hitresult _returnvalue) (`PlayerController.GetHitResultUnderCursorForObjects` (`GameplayStatics.GetPlayerController` 0) (`|MakeArray` "ObjectTypeQuery7" "ObjectTypeQuery9" :!type "EObjectTypeQuery Enum") true))
  (if _returnvalue
    (bind _output_get (set `self.HitLocation` (`.Location` (`GameplayStatics.BreakHitResult` _hitresult))))
    (bind _tileposition (`/Game/Blueprints/Macros/MacroLibrary.WorldToTilePos` _output_get))
    (bind _isempty_ (`/Game/Blueprints/BP_TileManager.CheckTile` (`self.TileManagerRef`) _tileposition))
    (return _isempty_ _tileposition _output_get)))

(fn `MultiTilePreview`
  (params (BuildingType :type "/Game/Blueprints/Structures/S_BuildingInfo Structure (by ref)") (Coordinate :type "/Game/Blueprints/Structures/IntVector2 Structure (by ref)") (Rotation :type "/Game/Blueprints/Enums/E_Direction Enum" :default "NewEnumerator0"))
  (bind (_x _y) (break `/Game/Blueprints/Structures/IntVector2` Coordinate))
  (bind (_x_2 _y_2) (break `/Game/Blueprints/Structures/IntVector2` (`.Size_15_4B26410D4E4F8DF384A9C0AB67D49E38` (break `/Game/Blueprints/Structures/S_BuildingInfo` BuildingType))))
  (bind _isvalidarea (`/Game/Blueprints/BP_TileManager.CheckTilesInArea` (`self.TileManagerRef`) Coordinate (`.Size_15_4B26410D4E4F8DF384A9C0AB67D49E38` (break `/Game/Blueprints/Structures/S_BuildingInfo` BuildingType)) Rotation))
  ;[1 1 1] X
  (for _index (range _x_2)
    ;[1 1 1] Y
    (for _index_2 (range _y_2)
      (bind _returnvalue (* _index (select `/Game/Blueprints/Enums/E_Direction` Rotation :`NewEnumerator0` 1 :`NewEnumerator1` -1 :`NewEnumerator2` -1 :`NewEnumerator3` 1)))
      (bind _returnvalue_2 (* _index_2 (select `/Game/Blueprints/Enums/E_Direction` Rotation :`NewEnumerator0` 1 :`NewEnumerator1` -1 :`NewEnumerator2` 1 :`NewEnumerator3` -1)))
      (bind _intvector2 (make `/Game/Blueprints/Structures/IntVector2` (+ _x (select `/Game/Blueprints/Enums/E_Direction` Rotation :`NewEnumerator0` _returnvalue :`NewEnumerator1` _returnvalue :`NewEnumerator2` _returnvalue_2 :`NewEnumerator3` _returnvalue_2)) (+ _y (select `/Game/Blueprints/Enums/E_Direction` Rotation :`NewEnumerator0` _returnvalue_2 :`NewEnumerator1` _returnvalue_2 :`NewEnumerator2` _returnvalue :`NewEnumerator3` _returnvalue))))
      (bind _returnvalue_3 (`|SpawnActorFromClass` "/Game/Blueprints/Tiles/BP_TilePreview.BP_TilePreview_C" (`KismetMathLibrary.MakeTransform` (`/Game/Blueprints/Macros/MacroLibrary.TileToWorldPos` _intvector2 (`/Game/Blueprints/BP_TileManager.TileSize` (`self.TileManagerRef`)) 50.0) (`KismetMathLibrary.MakeRotator` 0.0 0.0 (select `/Game/Blueprints/Enums/E_Direction` Rotation :`NewEnumerator1` 180.0 :`NewEnumerator2` -90.0 :`NewEnumerator3` 90.0 :!type "Float (single-precision)")) (1.1 1.1 1.1)) "AlwaysSpawn" "OverrideRootScale" null null))
      (`/Game/Blueprints/Tiles/BP_TilePreview.SetColour` _returnvalue_3 _isvalidarea)
      (`BlueprintMapLibrary.Map_Add` (`self.MultibuildingPreviewActors`) _intvector2 _returnvalue_3)))
  (return))

(fn `Place Row Of Tiles`
  (params (SelectionStartPos :type "/Game/Blueprints/Structures/IntVector2 Structure") (SelectionEndPos :type "/Game/Blueprints/Structures/IntVector2 Structure") (BuildingData :type "/Game/Blueprints/Structures/S_BuildingInfo Structure"))
  (bind _returnvalue (- SelectionStartPos_Y_5_2CE97EF04AC43C7EE518E4B20F9E68C5 SelectionEndPos_Y_5_2CE97EF04AC43C7EE518E4B20F9E68C5))
  (bind _returnvalue_2 (- SelectionStartPos_X_4_6582DAC54E23558CE2425DA215FE3DE3 SelectionEndPos_X_4_6582DAC54E23558CE2425DA215FE3DE3))
  (bind (_selectionstartpos_x _selectionstartpos_y) (break `/Game/Blueprints/Structures/IntVector2` (`self.SelectionStartPos`)))
  (bind (_selectionstartpos_x_2 _selectionstartpos_y_2) (break `/Game/Blueprints/Structures/IntVector2` (`self.SelectionStartPos`)))
  (bind _returnvalue_3 (`KismetMathLibrary.Abs_Int` _returnvalue_2))
  (bind _returnvalue_4 (`KismetMathLibrary.Abs_Int` _returnvalue))
  (bind _returnvalue_5 (< _returnvalue 0))
  (bind _returnvalue_6 (< _returnvalue_2 0))
  (bind _returnvalue_7 (== (`KismetMathLibrary.Max` _returnvalue_3 _returnvalue_4) _returnvalue_3))
  (if _returnvalue_7
    ;[1 1 1] If X is greater than Y
    (for _index (range (+ _returnvalue_3 1))
      (bind _direction (`self.DecideTileDirection` _returnvalue_7 _returnvalue_6))
      (`/Game/Blueprints/BP_TileManager.Place Tile` (`self.TileManagerRef`) (make `/Game/Blueprints/Structures/IntVector2` (+ _selectionstartpos_x (* _index (`KismetMathLibrary.SelectInt` 1 -1 _returnvalue_6))) _selectionstartpos_y) BuildingData _direction))
    (else
      ;[1 1 1] If Y is greater than X
      (for _index_2 (range (+ _returnvalue_4 1))
        (bind _direction_2 (`self.DecideTileDirection` _returnvalue_7 _returnvalue_5))
        (`/Game/Blueprints/BP_TileManager.Place Tile` (`self.TileManagerRef`) (make `/Game/Blueprints/Structures/IntVector2` _selectionstartpos_x_2 (+ _selectionstartpos_y_2 (* _index_2 (`KismetMathLibrary.SelectInt` 1 -1 _returnvalue_5)))) BuildingData _direction_2)))))

(fn `SpawnDestroyAreaPreview`
  (params (StartPos :type "/Game/Blueprints/Structures/IntVector2 Structure (by ref)") (EndPos :type "/Game/Blueprints/Structures/IntVector2 Structure"))
  (bind (_x _y) (break `/Game/Blueprints/Structures/IntVector2` StartPos))
  (bind (_x_2 _y_2) (break `/Game/Blueprints/Structures/IntVector2` EndPos))
  (bind (_x_3 _y_3) (break `/Game/Blueprints/Structures/IntVector2` StartPos))
  (bind _instancedstaticmesh (`/Game/Blueprints/BP_TileManager.InstancedStaticMesh` (`self.TileManagerRef`)))
  (bind (_x_4 _y_4) (break `/Game/Blueprints/Structures/IntVector2` (make `/Game/Blueprints/Structures/IntVector2` (`KismetMathLibrary.Clamp` (- (`KismetMathLibrary.Abs_Int` (`KismetMathLibrary.Max` _x _x_2)) (`KismetMathLibrary.Abs_Int` (`KismetMathLibrary.Min` _x _x_2))) 0 16) (`KismetMathLibrary.Clamp` (- (`KismetMathLibrary.Abs_Int` (`KismetMathLibrary.Max` _y _y_2)) (`KismetMathLibrary.Abs_Int` (`KismetMathLibrary.Min` _y _y_2))) 0 16))))
  (`InstancedStaticMeshComponent.ClearInstances` _instancedstaticmesh)
  ;[1 1 1] X
  (for _index (range (+ _x_4 1))
    ;[1 1 1] Y
    (for _index_2 (range (+ _y_4 1))
      (`InstancedStaticMeshComponent.AddInstance` _instancedstaticmesh (`KismetMathLibrary.MakeTransform` (`/Game/Blueprints/Macros/MacroLibrary.TileToWorldPos` (make `/Game/Blueprints/Structures/IntVector2` (+ (* _index (select `bool` (< _x _x_2) :`false` -1 :`true` 1)) _x_3) (+ (* _index_2 (select `bool` (< _y _y_2) :`false` -1 :`true` 1)) _y_3)) 100.0)) false)))
  (return))

(fn `SpawnPreviewRow`
  (params (SelectionStartPos :type "/Game/Blueprints/Structures/IntVector2 Structure") (SelectionEndPos :type "/Game/Blueprints/Structures/IntVector2 Structure") (TileType :type "StaticMesh Object Reference"))
  (bind _returnvalue (- SelectionStartPos_Y_5_2CE97EF04AC43C7EE518E4B20F9E68C5 SelectionEndPos_Y_5_2CE97EF04AC43C7EE518E4B20F9E68C5))
  (bind _returnvalue_2 (- SelectionStartPos_X_4_6582DAC54E23558CE2425DA215FE3DE3 SelectionEndPos_X_4_6582DAC54E23558CE2425DA215FE3DE3))
  (bind (_selectionstartpos_x _selectionstartpos_y) (break `/Game/Blueprints/Structures/IntVector2` (`self.SelectionStartPos`)))
  (bind (_selectionstartpos_x_2 _selectionstartpos_y_2) (break `/Game/Blueprints/Structures/IntVector2` (`self.SelectionStartPos`)))
  (bind _returnvalue_3 (`KismetMathLibrary.Abs_Int` _returnvalue_2))
  (bind _returnvalue_4 (`KismetMathLibrary.Abs_Int` _returnvalue))
  (bind _returnvalue_5 (< _returnvalue 0))
  (bind _returnvalue_6 (< _returnvalue_2 0))
  (bind _returnvalue_7 (== (`KismetMathLibrary.Max` _returnvalue_3 _returnvalue_4) _returnvalue_3))
  (if _returnvalue_7
    ;[1 1 1] If X is greater than Y
    (for _index (range (+ _returnvalue_3 1))
      (`self.DecideTileDirection` _returnvalue_7 _returnvalue_6)
      (bind _returnvalue_8 (+ _selectionstartpos_x (* _index (`KismetMathLibrary.SelectInt` 1 -1 _returnvalue_6))))
      (if (not (`BlueprintMapLibrary.Map_Contains` (`self.PreviewActors`) (make `/Game/Blueprints/Structures/IntVector2` _returnvalue_8 _selectionstartpos_y)))
        (bind _returnvalue_9 (`|SpawnActorFromClass` "/Game/Blueprints/Tiles/BP_TilePreview.BP_TilePreview_C" (`KismetMathLibrary.MakeTransform` (`/Game/Blueprints/Macros/MacroLibrary.TileToWorldPos` (make `/Game/Blueprints/Structures/IntVector2` _returnvalue_8 _selectionstartpos_y) 100.0 50.0) (`KismetMathLibrary.MakeRotator` 0.0 0.0 (select `/Game/Blueprints/Enums/E_Direction` "NewEnumerator0" :`NewEnumerator1` 180.0 :`NewEnumerator2` 270.0 :`NewEnumerator3` 90.0 :!type "Float (single-precision)"))) "AlwaysSpawn" "OverrideRootScale" null null))
        (`BlueprintMapLibrary.Map_Add` (`self.PreviewActors`) (make `/Game/Blueprints/Structures/IntVector2` _returnvalue_8 _selectionstartpos_y) _returnvalue_9)))
    (else
      ;[1 1 1] If Y is greater than X
      (for _index_2 (range (+ _returnvalue_4 1))
        (bind _direction (`self.DecideTileDirection` _returnvalue_7 _returnvalue_5))
        (bind _returnvalue_10 (+ _selectionstartpos_y_2 (* _index_2 (`KismetMathLibrary.SelectInt` 1 -1 _returnvalue_5))))
        (if (not (`BlueprintMapLibrary.Map_Contains` (`self.PreviewActors`) (make `/Game/Blueprints/Structures/IntVector2` _selectionstartpos_x_2 _returnvalue_10)))
          (bind _returnvalue_11 (`|SpawnActorFromClass` "/Game/Blueprints/Tiles/BP_TilePreview.BP_TilePreview_C" (`KismetMathLibrary.MakeTransform` (`/Game/Blueprints/Macros/MacroLibrary.TileToWorldPos` (make `/Game/Blueprints/Structures/IntVector2` _selectionstartpos_x_2 _returnvalue_10) 100.0 50.0) (`KismetMathLibrary.MakeRotator` 0.0 0.0 (select `/Game/Blueprints/Enums/E_Direction` _direction :`NewEnumerator1` 180.0 :`NewEnumerator2` 270.0 :`NewEnumerator3` 90.0 :!type "Float (single-precision)"))) "AlwaysSpawn" "OverrideRootScale" null null))
          (`BlueprintMapLibrary.Map_Add` (`self.PreviewActors`) (make `/Game/Blueprints/Structures/IntVector2` _selectionstartpos_x_2 _returnvalue_10) _returnvalue_11))))))

(fn `UserConstructionScript`)