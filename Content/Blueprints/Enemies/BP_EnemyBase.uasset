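; Base enemy Blueprint that moves at a set speed, takes damage until destroyed and attacks nearby tiles.
; A looping one-second timer damages the tiles of BP_TileBase actors overlapping its AttackBox and spawns a hit effect on each.
; A timeline procedurally swings arm and leg pivots in opposite pairs, with play rate scaled by current velocity.
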(event `self.ReceiveBeginPlay`
  (bind _returnvalue (`KismetMathLibrary.MapRangeClamped` (`KismetMathLibrary.VSize` (`self.GetVelocity`)) 0.0 (`self.MoveSpeed`) 0.0 (`self.AnimationSpeed`)))
  (`ActorComponent.SetComponentTickEnabled` (`self.NavigationInvoker`) true)
  (`KismetSystemLibrary.K2_SetTimerDelegate` (delegate `Attack`) 1.0 true)
  (set `CharacterMovementComponent.MaxWalkSpeed` (`self.MoveSpeed`) (`self.CharacterMovement`))
  ;[1 1 1] Movement animation
  (bind (_direction _swing) (`Timeline|AnimationTimeline` :!via `PlayFromStart`)
    (:`Update`
      (`TimelineComponent.SetPlayRate` (`self.AnimationTimeline`) (`KismetMathLibrary.SelectFloat` 0.0 _returnvalue (< _returnvalue 0.25)))
      (bind _returnvalue_2 (* (`self.AnimationAmount`) (`GameplayStatics.GetWorldDeltaSeconds`) _swing))
      (`SceneComponent.K2_SetRelativeRotation` (`self.ArmPivotR`) (`KismetMathLibrary.MakeRotator` _returnvalue_2) false false)
      (`SceneComponent.K2_SetRelativeRotation` (`self.LegPivotL`) (`KismetMathLibrary.MakeRotator` _returnvalue_2) false false)
      (`SceneComponent.K2_SetRelativeRotation` (`self.ArmPivotL`) (`KismetMathLibrary.MakeRotator` (* _returnvalue_2 -1.0)) false false)
      (`SceneComponent.K2_SetRelativeRotation` (`self.LegPivotR`) (`KismetMathLibrary.MakeRotator` (* _returnvalue_2 -1.0)) false false))))

(event `Attack`
  (for _array_element (`PrimitiveComponent.GetOverlappingActors` (`self.AttackBox`) "/Game/Blueprints/Tiles/BP_TileBase.BP_TileBase_C")
    (bind _tileref (message `/Game/Blueprints/Interfaces/BPI_Tile.GetTile` _array_element))
    (`/Engine/EditorBlueprintResources/StandardMacros.IsValid` _tileref
      (:`Is Valid`
        (`NiagaraFunctionLibrary.SpawnSystemAtLocation` "/Game/ParticleEffects/NS_ProjectileHit.NS_ProjectileHit" (`self.K2_GetActorLocation` _tileref))
        (`/Game/Blueprints/Tiles/BP_TileBase.DamageTile` _tileref (`self.Damage`))))))

(event `/Game/Blueprints/Interfaces/BPI_Enemy.DoDamage`
  (params (Damage :type Integer))
  (bind _output_get (set `self.Health` (- (`self.Health`) Damage)))
  (if (<= _output_get 0)
    (`self.K2_DestroyActor`)))

(fn `UserConstructionScript`)