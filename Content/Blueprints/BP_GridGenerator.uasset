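; Grid generator that builds a tile map for what appears to be a mining/factory game.
; BeginPlay creates a seeded FastNoise wrapper, never sampled here, and spawns a grid of solid walls.
; Helpers define random-walk caves and resource veins, floating-wall cleanup, index-based tile swapping, and a central core with four lights.
; The generation sequence, tile registration and SwapTile's replacement bookkeeping are disconnected, so only the wall grid generates at BeginPlay.
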(event `self.ReceiveBeginPlay`
  (bind _spacing (`self.Spacing`))
  (`self.SetupNoise`)
  (for _index (range (`self.NumYTiles`))
    (for _index_2 (range (`self.NumXTiles`))
      (bind _returnvalue (`|SpawnActorFromClass` "/Game/Blueprints/Tiles/BP_SolidWall.BP_SolidWall_C" (`KismetMathLibrary.MakeTransform` (`KismetMathLibrary.MakeVector` (- (* (`KismetMathLibrary.Conv_IntToDouble` _index) _spacing) (`self.Offset`)) (- (* (`KismetMathLibrary.Conv_IntToDouble` _index_2) _spacing) (`self.Offset`)))) "Undefined" "OverrideRootScale" null null)))))

(event `SpawnCore`
  (bind _centerindex (`self.FindCenter` (`self.NumXTiles`) (`self.NumYTiles`)))
  (bind (_success_ _spawnedtile) (`self.SwapTile` "/Game/Blueprints/Tiles/BP_Core.BP_Core_C" _centerindex))
  (if _success_
    (set `self.CoreRef` _spawnedtile)
    (`|ExecutionSequence`
      (:`then_0`
        (`self.SwapTile` "/Game/Blueprints/Tiles/BP_Light.BP_Light_C" (- (+ _centerindex 5) (* (`self.NumXTiles`) 5))))
      (:`then_1`
        (`self.SwapTile` "/Game/Blueprints/Tiles/BP_Light.BP_Light_C" (- (+ _centerindex -5) (* (`self.NumXTiles`) 5))))
      (:`then_2`
        (`self.SwapTile` "/Game/Blueprints/Tiles/BP_Light.BP_Light_C" (+ (+ _centerindex 5) (* (`self.NumXTiles`) 5))))
      (:`then_3`
        (`self.SwapTile` "/Game/Blueprints/Tiles/BP_Light.BP_Light_C" (+ (+ _centerindex -5) (* (`self.NumXTiles`) 5)))))))

(fn `FindCenter`
  (params (X :type Integer) (Y :type Integer))
  (returns (CenterIndex :type Integer))
  (return (/ (* X Y) 2)))

(fn `GenerateCaves`
  (params (NumCaveTiles :type Integer) (StartPointIndex :type Integer))
  (locals (StartPoint :type Integer) (CurrentPoint :type Integer) (Direction :type "/Game/Blueprints/Enums/E_Direction Enum") (CurrentTiles :type Integer :default 0) (TotalTiles :type Integer :default 20))
  (set `local.TotalTiles` NumCaveTiles)
  (bind _output_get (set `local.StartPoint` StartPointIndex))
  (set `local.CurrentPoint` _output_get)
  (while (not (>= (`local.CurrentTiles`) (`local.TotalTiles`)))
    (set `local.Direction` (select `int` (`KismetMathLibrary.RandomIntegerInRange` 0 3) :`0` "NewEnumerator0" :`1` "NewEnumerator1" :`2` "NewEnumerator2" :`3` "NewEnumerator3" :!type "/Game/Blueprints/Enums/E_Direction Enum"))
    (bind _outindex (`self.GetTileInDir` (`local.CurrentPoint`) (`local.Direction`)))
    (bind _inbounds (`self.IsInBounds` _outindex))
    (if _inbounds
      (bind _output_get_2 (set `local.CurrentPoint` _outindex))
      (`/Engine/EditorBlueprintResources/StandardMacros.IncrementInt` (`local.CurrentTiles`)
        (:`  `
          (`self.SwapTile` "/Game/Blueprints/Tiles/BP_TileBase.BP_TileBase_C" (`local.CurrentPoint`)))))))

(fn `GenerateResources`
  (params (ResourcesPerVein :type Integer) (ResourceType :type "/Game/Blueprints/Tiles/E_ResourceTypes Enum" :default "NewEnumerator3"))
  (locals (StartPoint :type Integer) (CurrentPoint :type Integer) (CurrentResources :type Integer) (Direction :type "/Game/Blueprints/Enums/E_Direction Enum") (Type :type "/Game/Blueprints/Tiles/E_ResourceTypes Enum" :default "NewEnumerator3"))
  (set `local.Type` ResourceType)
  (bind _output_get (set `local.StartPoint` (`KismetMathLibrary.RandomIntegerInRange` 0 (`self.NumOfIndices`))))
  (set `local.CurrentPoint` _output_get)
  (while (not (>= (`local.CurrentResources`) ResourcesPerVein))
    (set `local.Direction` (select `int` (`KismetMathLibrary.RandomIntegerInRange` 0 3) :`0` "NewEnumerator0" :`1` "NewEnumerator1" :`2` "NewEnumerator2" :`3` "NewEnumerator3" :!type "/Game/Blueprints/Enums/E_Direction Enum"))
    (bind _outindex (`self.GetTileInDir` (`local.CurrentPoint`) (`local.Direction`)))
    (bind _inbounds (`self.IsInBounds` _outindex))
    (if _inbounds
      (bind _output_get_2 (set `local.CurrentPoint` _outindex))
      (`/Engine/EditorBlueprintResources/StandardMacros.IncrementInt` (`local.CurrentResources`)
        (:`  `
          (`BlueprintMapLibrary.Map_Add` (`self.ResourceTypes`) (`local.CurrentPoint`) (`local.Type`)))))))

(fn `GetNeighborTiles`
  (params (Index :type Integer))
  (returns (UpTile :type "/Game/Blueprints/Tiles/BP_TileBase Object Reference") (DownTile :type "/Game/Blueprints/Tiles/BP_TileBase Object Reference") (LeftTile :type "/Game/Blueprints/Tiles/BP_TileBase Object Reference") (RightTile :type "/Game/Blueprints/Tiles/BP_TileBase Object Reference") (UpLeftTile :type "/Game/Blueprints/Tiles/BP_TileBase Object Reference") (UpRightTile :type "/Game/Blueprints/Tiles/BP_TileBase Object Reference") (DownLeftTile :type "/Game/Blueprints/Tiles/BP_TileBase Object Reference") (DownRightTile :type "/Game/Blueprints/Tiles/BP_TileBase Object Reference") (Tiles :type "Array of /Game/Blueprints/Tiles/BP_TileBase Object Reference") (Indices :type "Array of Integer"))
  (bind _returnvalue (+ Index 1))
  (bind _returnvalue_2 (+ Index -1))
  (bind _tilerefs (`self.TileRefs`))
  (bind _numxtiles (`self.NumXTiles`))
  (bind _tilerefs_2 (`self.TileRefs`))
  (bind _numxtiles_2 (`self.NumXTiles`))
  (bind _value (`BlueprintMapLibrary.Map_Find` _tilerefs_2 _returnvalue))
  (bind _value_2 (`BlueprintMapLibrary.Map_Find` _tilerefs_2 _returnvalue_2))
  (bind _returnvalue_3 (- Index _numxtiles_2))
  (bind _returnvalue_4 (+ Index _numxtiles_2))
  (bind _returnvalue_5 (- (+ Index _numxtiles) 1))
  (bind _returnvalue_6 (- (- Index _numxtiles) 1))
  (bind _value_3 (`BlueprintMapLibrary.Map_Find` _tilerefs_2 _returnvalue_4))
  (bind _value_4 (`BlueprintMapLibrary.Map_Find` _tilerefs_2 _returnvalue_3))
  (bind _returnvalue_7 (+ (- Index _numxtiles) 1))
  (bind _returnvalue_8 (+ (+ _numxtiles Index) 1))
  (bind _value_5 (`BlueprintMapLibrary.Map_Find` _tilerefs _returnvalue_6))
  (bind _value_6 (`BlueprintMapLibrary.Map_Find` _tilerefs _returnvalue_7))
  (bind _value_7 (`BlueprintMapLibrary.Map_Find` _tilerefs _returnvalue_8))
  (bind _value_8 (`BlueprintMapLibrary.Map_Find` _tilerefs _returnvalue_5))
  (return _value_3 _value_4 _value_2 _value _value_8 _value_7 _value_5 _value_6 (`|MakeArray` _value_3 _value_4 _value_2 _value _value_8 _value_5 _value_7 _value_6) (`|MakeArray` _returnvalue_4 _returnvalue_3 _returnvalue_2 _returnvalue _returnvalue_5 _returnvalue_6 _returnvalue_8 _returnvalue_7)))

(fn `GetTileInDir`
  (params (InIndex :type Integer) (Direction :type "/Game/Blueprints/Enums/E_Direction Enum" :default "NewEnumerator0"))
  (returns (OutIndex :type Integer) (Tile :type "/Game/Blueprints/Tiles/BP_TileBase Object Reference"))
  (bind _returnvalue (+ InIndex -1))
  (bind _returnvalue_2 (+ InIndex 1))
  (bind _tilerefs (`self.TileRefs`))
  (bind _numxtiles (`self.NumXTiles`))
  (bind _returnvalue_3 (- InIndex _numxtiles))
  (bind _returnvalue_4 (+ InIndex _numxtiles))
  (return (select `/Game/Blueprints/Enums/E_Direction` Direction :`NewEnumerator0` _returnvalue_4 :`NewEnumerator1` _returnvalue_3 :`NewEnumerator2` _returnvalue :`NewEnumerator3` _returnvalue_2) (select `/Game/Blueprints/Enums/E_Direction` Direction :`NewEnumerator0` (`BlueprintMapLibrary.Map_Find` _tilerefs _returnvalue_4) :`NewEnumerator1` (`BlueprintMapLibrary.Map_Find` _tilerefs _returnvalue_3) :`NewEnumerator2` (`BlueprintMapLibrary.Map_Find` _tilerefs _returnvalue) :`NewEnumerator3` (`BlueprintMapLibrary.Map_Find` _tilerefs _returnvalue_2))))

(fn `GetTouchingTiles`
  (params (Index :type Integer))
  (returns (UpTile :type "/Game/Blueprints/Tiles/BP_TileBase Object Reference") (DownTile :type "/Game/Blueprints/Tiles/BP_TileBase Object Reference") (LeftTile :type "/Game/Blueprints/Tiles/BP_TileBase Object Reference") (RightTile :type "/Game/Blueprints/Tiles/BP_TileBase Object Reference"))
  (bind _tilerefs (`self.TileRefs`))
  (bind _numxtiles (`self.NumXTiles`))
  (return (`BlueprintMapLibrary.Map_Find` _tilerefs (+ Index _numxtiles)) (`BlueprintMapLibrary.Map_Find` _tilerefs (- Index _numxtiles)) (`BlueprintMapLibrary.Map_Find` _tilerefs (+ Index -1)) (`BlueprintMapLibrary.Map_Find` _tilerefs (+ Index 1))))

(fn `IsInBounds`
  (params (InIndex :type Integer))
  (returns (InBounds :type Boolean))
  (return (or (>= InIndex 0) (<= InIndex (`self.NumOfIndices`)))))

(fn `RemoveFloatingTiles`
  (bind _values (`BlueprintMapLibrary.Map_Values` (`self.TileRefs`)))
  (for (_array_element _array_index) _values
    (if (== (`GameplayStatics.GetObjectClass` _array_element) "/Game/Blueprints/Tiles/BP_SolidWall.BP_SolidWall_C")
      (bind (_uptile _downtile _lefttile _righttile) (`self.GetTouchingTiles` _array_index))
      (if (and (!= _uptile "/Game/Blueprints/Tiles/BP_SolidWall.BP_SolidWall") (!= _downtile "/Game/Blueprints/Tiles/BP_SolidWall.BP_SolidWall") (!= _lefttile "/Game/Blueprints/Tiles/BP_SolidWall.BP_SolidWall") (!= _righttile "/Game/Blueprints/Tiles/BP_SolidWall.BP_SolidWall"))
        (`self.SwapTile` "/Game/Blueprints/Tiles/BP_TileBase.BP_TileBase_C" _array_index)
        (return)))))

(fn `SetupNoise`
  (bind _returnvalue (`|GenericCreateObject` self "/Script/FastNoiseGenerator.FastNoiseWrapper"))
  (bind _output_get (set `self.FastNoiseWrapper` _returnvalue))
  (`FastNoiseWrapper.SetupFastNoise` _output_get "Simplex" (`self.Seed`) 0.01 "Quintic" "FBM" 3 2.0 0.5 0.45 "Euclidean" "CellValue")
  (return))

(fn `SwapTile`
  (params (`New Tile` :type "/Game/Blueprints/Tiles/BP_TileBase Class Reference") (Index :type "Integer (by ref)") (Direction :type "/Game/Blueprints/Enums/E_Direction Enum" :default "NewEnumerator0"))
  (returns (`Success?` :type Boolean) (SpawnedTile :type "/Game/Blueprints/Tiles/BP_TileBase Object Reference"))
  (locals (OldTile :type "/Game/Blueprints/Tiles/BP_TileBase Object Reference"))
  (bind (_value _returnvalue) (`BlueprintMapLibrary.Map_Find` (`self.TileRefs`) Index))
  (if _returnvalue
    (set `local.OldTile` _value)
    (bind _output_get (set `self.TileIndex` Index))
    (bind _returnvalue_2 (`|SpawnActorFromClass` `New Tile` (`KismetMathLibrary.MakeTransform` (.location (`self.GetTransform` _value)) (`KismetMathLibrary.MakeRotator` 0.0 0.0 (select `byte` Direction :`0` 0.0 :`1` 90.0 :`2` 180.0 :`3` 270.0)) (.scale (`self.GetTransform` _value))) "Undefined" "OverrideRootScale" null null))
    (else
      (`KismetSystemLibrary.PrintString` "Error")
      (return false null))))

(fn `UpdateResourceTiles`
  (bind _values (`BlueprintMapLibrary.Map_Values` (`self.ResourceTypes`)))
  (for (_array_element _array_index) _values
    (if (`|EnumInequality` _array_element "NewEnumerator3")
      (if (`.ReturnValue` (`BlueprintMapLibrary.Map_Find` (`self.TileRefs`) _array_index))
        _))))

(fn `UserConstructionScript`)