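; Inventory component that stores items in an Items array and exposes functions to add and remove them.
; Separate check functions report whether the array is below Capacity or holds any items.
; Adding appends without checking Capacity itself, while removal takes no item argument and drops the last entry if the array is not empty.
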(fn `AddToInventory`
  (params (NewItem :type "/Game/Blueprints/Structures/S_ItemData Structure (by ref)"))
  (returns (`Added?` :type Boolean))
  (`KismetArrayLibrary.Array_Add` (`self.Items`) NewItem)
  (return true))

(fn `Can Add To Inventory?`
  (returns (CanAdd :type Boolean))
  (if (< (`KismetArrayLibrary.Array_Length` (`self.Items`)) (`self.Capacity`))
    (return true)
    (else
      (return false))))

(fn `Can Remove From Inventory?`
  (returns (CanRemove :type Boolean))
  (if (> (`KismetArrayLibrary.Array_Length` (`self.Items`)) 0)
    (return true)
    (else
      (return false))))

(fn `RemoveFromInventory`
  (returns (`Removed?` :type Boolean))
  (bind _items (`self.Items`))
  (if (`KismetArrayLibrary.Array_IsNotEmpty` _items)
    (`KismetArrayLibrary.Array_Remove` _items (`KismetArrayLibrary.Array_LastIndex` _items))
    (return true)))