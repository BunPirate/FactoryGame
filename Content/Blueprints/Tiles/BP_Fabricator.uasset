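; Fabricator tile for a conveyor factory that crafts an item from a DT_Items recipe, with a crafting window opened on interact.
; It accepts and destroys items matching remaining recipe inputs.
; Once none remain, Tick spawns the output and, if the output tile accepts it, moves it there and refills the needed list.
; A timeline spins three gears while active, a state that a timer clears after activation.
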(event `self.Interact`
  ;[1 1 1] Set the desired item to produce
  (bind _playerref (message `/Game/Blueprints/Player/BPI_Player.GetPlayer` (`GameplayStatics.GetPlayerPawn` 0)))
  (`/Game/Blueprints/UI/W_HUD.OpenCraftingWindow` (`/Game/Blueprints/Player/BP_PlayerController.HudRef` (`/Game/Blueprints/Player/BP_PlayerPawn.PlayerController` _playerref)) self))

(event `SetRecipe`
  (params (ItemData :type "/Game/Blueprints/Structures/S_ItemData Structure"))
  (bind (_name _mesh _icon _rownumber _fabricationtype _requirements) (break `/Game/Blueprints/Structures/S_ItemData` ItemData))
  (bind _allowedinputitems (`self.AllowedInputItems`))
  ;[1 1 1] Set the desired item to produce
  (`KismetArrayLibrary.Array_Clear` _allowedinputitems)
  (`KismetArrayLibrary.Array_Resize` _allowedinputitems)
  (for (_array_element _array_index) _requirements
    (`KismetArrayLibrary.Array_Set` (`self.AllowedInputItems`) _array_index (`KismetStringLibrary.Conv_StringToInt` _array_element) true))
  (set `self.OutputItem` _rownumber))

(event `ActivateFabricator`
  (set `self.IsActive` true)
  (`KismetSystemLibrary.K2_SetTimerDelegate` (delegate `DeactivateFabricator`) 6.0))

(event `DeactivateFabricator`
  (set `self.IsActive` false))

(event `self.ReceiveBeginPlay`
  (bind _returnvalue (`|GetDataTableRow` "/Game/Blueprints/Datatables/DT_Items.DT_Items" "4")
    (:`then`
      (`self.SetRecipe` _returnvalue)
      (set `self.NeededItems` (`self.AllowedInputItems`))
      (`Timeline|Rotat`
        (:`Update`
          (if (`self.IsActive`)
            (`SceneComponent.K2_AddRelativeRotation` (`self.GearPivot2`) (struct :`Roll` 0.25) false false)
            (`SceneComponent.K2_AddRelativeRotation` (`self.GearPivot1`) (struct :`Roll` 0.25) false false)
            (`SceneComponent.K2_AddRelativeRotation` (`self.GearPivot3`) (struct :`Roll` -0.35) false false)))))))

(event `self.ReceiveTick`
  (params (DeltaSeconds :type "Float (single-precision)"))
  (bind _returnvalue (`SceneComponent.K2_GetComponentLocation` (`self.OutputPos`)))
  (if (`KismetArrayLibrary.Array_IsEmpty` (`self.NeededItems`))
    (bind _returnvalue_2 (`|GetDataTableRow` "/Game/Blueprints/Datatables/DT_Items.DT_Items" (`KismetStringLibrary.Conv_StringToName` (`KismetStringLibrary.Conv_IntToString` (`self.OutputItem`))))
      (:`then`
        (bind _tileref (message `/Game/Blueprints/Interfaces/BPI_Tile.GetTile` (`BlueprintMapLibrary.Map_Find` (`/Game/Blueprints/BP_TileManager.TileActors` (`self.TileManagerRef`)) (`/Game/Blueprints/Macros/MacroLibrary.WorldToTilePos` _returnvalue))))
        (bind _output_get (set `self.TargetTile` _tileref))
        (`self.SpawnItemOnConveyor` self _returnvalue_2)
        (bind _canadd_ (message `/Game/Blueprints/Interfaces/BPI_Tile.CanAddItemToTile` _output_get (`self.CurrentItem`)))
        (if _canadd_
          (`/Game/Blueprints/Items/BP_ItemBase.MoveItem` (`self.CurrentItem`) self _output_get (`SceneComponent.K2_GetComponentLocation` (`self.Direction`)) _returnvalue)
          (set `/Game/Blueprints/Tiles/BP_TileBase.IsReserved` true _output_get)
          (set `self.NeededItems` (`self.AllowedInputItems`)))))))

(event `self.AddItemToTile`
  (params (NewItem :type "/Game/Blueprints/Items/BP_ItemBase Object Reference"))
  (bind (_itemdata_name _itemdata_mesh _itemdata_icon _itemdata_rownumber) (break `/Game/Blueprints/Structures/S_ItemData` (`/Game/Blueprints/Items/BP_ItemBase.ItemData` NewItem)))
  (bind _neededitems (`self.NeededItems`))
  (if (`KismetArrayLibrary.Array_Contains` _neededitems _itemdata_rownumber)
    (`KismetArrayLibrary.Array_RemoveItem` _neededitems _itemdata_rownumber)
    (`KismetArrayLibrary.Array_Add` (`self.CurrentItems`) _itemdata_rownumber))
  (`/Engine/EditorBlueprintResources/StandardMacros.IsValid` NewItem
    (:`Is Valid`
      (`/Game/Blueprints/Items/BP_ItemBase.DestroyItem` NewItem))))

(event `self.SpawnItemOnConveyor`
  (params (NewItem :type "/Game/Blueprints/Structures/S_ItemData Structure"))
  (bind _returnvalue (`|SpawnActorFromClass` "/Game/Blueprints/Items/BP_ItemBase.BP_ItemBase_C" (`KismetMathLibrary.MakeTransform` (`SplineComponent.GetLocationAtDistanceAlongSpline` (`self.Spline`) 50.0 "World")) "Undefined" "OverrideRootScale" null null))
  (bind _itemref (message `/Game/Blueprints/Items/BPI_Item.GetItem` _returnvalue))
  (bind _output_get (set `self.CurrentItem` _itemref))
  (`/Game/Blueprints/Items/BP_ItemBase.InitItemStats` _output_get NewItem))

(fn `CanAddItemToTile`
  (params (NewItem :type "/Game/Blueprints/Items/BP_ItemBase Object Reference"))
  (returns (`CanAdd?` :type Boolean))
  (bind (_itemdata_name _itemdata_mesh _itemdata_icon _itemdata_rownumber) (break `/Game/Blueprints/Structures/S_ItemData` (`/Game/Blueprints/Items/BP_ItemBase.ItemData` NewItem)))
  (if (`KismetArrayLibrary.Array_Contains` (`self.NeededItems`) _itemdata_rownumber)
    (return true)
    (else
      (return false))))

(fn `DoneMoving`
  (`self.AddItemToTile` (`self.TargetTile`) (`self.CurrentItem`))
  (set `self.CurrentItem` null)
  (set `self.IsReserved` false)
  (return))

(fn `GetTile`
  (returns (TileRef :type "/Game/Blueprints/Tiles/BP_TileBase Object Reference"))
  (return self))

(fn `UserConstructionScript`)