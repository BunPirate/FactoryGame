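; BP_Turret is an automated turret that tracks and fires at the nearest BP_EnemyBase actor within its SightRadius.
; Each tick it picks the closest overlapping enemy, then uses interpolated look-at rotation to set yaw on Cube and pitch on Cube1.
; A looping timer started at BeginPlay spawns BP_ProjectileBase at FirePoint whenever a valid target exists.
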(event `self.ReceiveTick`
  (params (DeltaSeconds :type "Float (single-precision)"))
  (bind _cube (`self.Cube`))
  (`parent.ReceiveTick` DeltaSeconds)
  (bind _closestenemyactor (`self.GetClosestEnemy`))
  (bind _output_get (set `self.HasTarget` (`KismetSystemLibrary.IsValid` _closestenemyactor)))
  (if _output_get
    (bind (_returnvalue_roll _returnvalue_pitch _returnvalue_yaw) (`KismetMathLibrary.BreakRotator` (`KismetMathLibrary.RInterpTo` (`SceneComponent.RelativeRotation` _cube) (`KismetMathLibrary.FindRelativeLookAtRotation` (`self.GetTransform`) (`self.K2_GetActorLocation` _closestenemyactor)) DeltaSeconds 5.0)))
    (`SceneComponent.K2_SetRelativeRotation` _cube (`KismetMathLibrary.MakeRotator` 0.0 0.0 _returnvalue_yaw) false false)
    (`SceneComponent.K2_SetRelativeRotation` (`self.Cube1`) (`KismetMathLibrary.MakeRotator` 0.0 _returnvalue_pitch) false false)))

(event `self.ReceiveBeginPlay`
  (`KismetSystemLibrary.K2_SetTimerDelegate` (delegate `Shoot`) 0.2 true))

(event `Shoot`
  (bind (_returnvalue_location _returnvalue_rotation) (`KismetMathLibrary.BreakTransform` (`SceneComponent.K2_GetComponentToWorld` (`self.FirePoint`))))
  (if (`self.HasTarget`)
    (`|SpawnActorFromClass` "/Game/Blueprints/Projectiles/BP_ProjectileBase.BP_ProjectileBase_C" (`KismetMathLibrary.MakeTransform` _returnvalue_location _returnvalue_rotation) "AlwaysSpawn" "OverrideRootScale" null null)))

(fn `GetClosestEnemy`
  (returns (ClosestEnemyActor :type "Actor Object Reference"))
  (locals (ClosestDistance :type "Float (double-precision)" :default 9999999999999.0) (ClosestEnemy :type "Actor Object Reference"))
  (for _array_element (`PrimitiveComponent.GetOverlappingActors` (`self.SightRadius`) "/Game/Blueprints/Enemies/BP_EnemyBase.BP_EnemyBase_C")
    (bind _returnvalue (`KismetMathLibrary.Vector_Distance` (`self.K2_GetActorLocation` _array_element) (`self.K2_GetActorLocation`)))
    (if (< _returnvalue (`local.ClosestDistance`))
      (set `local.ClosestDistance` _returnvalue)
      (set `local.ClosestEnemy` _array_element)))
  (return (`local.ClosestEnemy`)))

(fn `UserConstructionScript`
  (`parent.UserConstructionScript`))