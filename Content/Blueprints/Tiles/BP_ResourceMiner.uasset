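; BP_ResourceMiner is a tile actor that produces a configured item and feeds it to the neighboring tile it faces.
; On BeginPlay it caches the item from the DT_Items data table using its row name.
; Every tick, with no timer of its own, it finds the tile ahead in the tile manager's coordinate map.
; If that tile's GetTileMessage returns a valid result, it sends a SpawnItemOnConveyorMessage carrying the item.
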(event `self.ReceiveBeginPlay`
  (bind _returnvalue (`|GetDataTableRow` "/Game/Blueprints/Datatables/DT_Items.DT_Items" (`self.ItemToProduceRowName`))
    (:`then`
      (set `self.ItemToProduce` _returnvalue))))

(event `self.ReceiveTick`
  (params (DeltaSeconds :type "Float (single-precision)"))
  (bind (_value _returnvalue) (`BlueprintMapLibrary.Map_Find` (`/Game/Blueprints/BP_TileManager.TileActors` (`self.TileManagerRef`)) (`/Game/Blueprints/Macros/MacroLibrary.GetCoordInDirection` (`self.Coordinate`) (`self.TileDirection`))))
  (if _returnvalue
    (bind _tileref (message `/Game/Blueprints/Interfaces/BPI_Tile.GetTile` _value))
    (`/Engine/EditorBlueprintResources/StandardMacros.IsValid` _tileref
      (:`Is Valid`
        (message `/Game/Blueprints/Interfaces/BPI_Tile.SpawnItemOnConveyor` _value (`self.ItemToProduce`))))))

(fn `UserConstructionScript`
  (`parent.UserConstructionScript`))