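; BP_TileBase is the base Blueprint for grid tiles, initialized with references to a tile manager and level generator.
; InitializeTile clears neighbours, stores direction and coordinate, and sets actor ticking and interval from the tile's own variables.
; AddItemtoTile, CanAddItemToTile and DoneMoving are stubs with no behavior, with item acceptance false by default, while GetTile returns the tile itself.
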(event `/Game/Blueprints/Interfaces/BPI_Tile.InitializeTile`
  (params (TileManager :type "/Game/Blueprints/BP_TileManager Object Reference") (LevelGenerator :type "/Game/Blueprints/BP_LevelGenerator Object Reference") (Coordinate :type "/Game/Blueprints/Structures/IntVector2 Structure") (Direction :type "/Game/Blueprints/Enums/E_Direction Enum" :default "NewEnumerator0"))
  (`|ExecutionSequence`
    (:`then_0`
      (set `self.Neighbours` (struct)))
    (:`then_1`
      (set `self.TileDirection` Direction))
    (:`then_2`
      (`|ExecutionSequence`
        (:`then_0`
          (set `self.TileManagerRef` TileManager))
        (:`then_1`
          (set `self.LevelGeneratorRef` LevelGenerator))
        (:`then_2`
          (set `self.Coordinate` Coordinate))
        (:`then_3`
          (`self.SetActorTickEnabled` (`self.DoesTick`)))
        (:`then_4`
          (`self.SetActorTickInterval` (`self.TickInterval`)))))))

(event `self.ReceiveTick`
  (params (DeltaSeconds :type "Float (single-precision)")))

(event `/Game/Blueprints/Interfaces/BPI_Tile.AddItemToTile`
  (params (NewItem :type "/Game/Blueprints/Items/BP_ItemBase Object Reference")))

(fn `CanAddItemToTile`
  (returns (`CanAdd?` :type Boolean))
  (return false))

(fn `DoneMoving`
  (return))

(fn `GetTile`
  (returns (TileRef :type "/Game/Blueprints/Tiles/BP_TileBase Object Reference"))
  (return self))

(fn `UserConstructionScript`)