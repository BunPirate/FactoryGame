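; BP_Core is the core tile that serves as the player's item stockpile; its destruction loses the game through BP_Gamemode.
; It seeds starting stock from DT_Items, then absorbs allowed incoming items, storing their data and destroying the item objects.
; Stock is a flat array with one entry per unit, counted and removed by row number, and pushed to the HUD for display.
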(event `/Game/Blueprints/Interfaces/BPI_Tile.AddItemToTile`
  (params (NewItem :type "/Game/Blueprints/Items/BP_ItemBase Object Reference"))
  (`KismetArrayLibrary.Array_Add` (`self.Items`) (`/Game/Blueprints/Items/BP_ItemBase.ItemData` NewItem))
  (`/Engine/EditorBlueprintResources/StandardMacros.IsValid` NewItem
    (:`Is Valid`
      (`/Game/Blueprints/Items/BP_ItemBase.DestroyItem` NewItem))
    (:`Is Not Valid`
      _))
  (`/Game/Blueprints/UI/W_HUD.UpdateItems` (`self.Hud Ref`) (`self.Items`)))

(event `self.ReceiveBeginPlay`
  ;[1 1 1] Adds starting Items
  (`self.AddManyItems` 2 250)
  (`self.AddManyItems` 6 250)
  (`KismetSystemLibrary.Delay` 0.2)
  (bind _playerref (message `/Game/Blueprints/Player/BPI_Player.GetPlayer` (`GameplayStatics.GetPlayerPawn` 0)))
  (`/Engine/EditorBlueprintResources/StandardMacros.IsValid` _playerref
    (:`Is Valid`
      (bind _output_get (set `self.Hud Ref` (`/Game/Blueprints/Player/BP_PlayerController.HudRef` (`/Game/Blueprints/Player/BP_PlayerPawn.PlayerController` _playerref))))
      (`/Game/Blueprints/UI/W_HUD.UpdateItems` _output_get (`self.Items`)))))

(event `UpdateUIItems`
  (`/Game/Blueprints/UI/W_HUD.UpdateItems` (`self.Hud Ref`) (`self.Items`)))

(fn `AddManyItems`
  (params (ItemID :type Integer) (Amount :type Integer))
  (bind _returnvalue (`|GetDataTableRow` "/Game/Blueprints/Datatables/DT_Items.DT_Items" (`KismetStringLibrary.Conv_StringToName` (`KismetStringLibrary.Conv_IntToString` ItemID)))
    (:`then`
      (for _ (range Amount)
        (`KismetArrayLibrary.Array_Add` (`self.Items`) _returnvalue)))))

(fn `CanAddItemToTile`
  (params (NewItem :type "/Game/Blueprints/Items/BP_ItemBase Object Reference"))
  (returns (`CanAdd?` :type Boolean))
  (bind (_itemdata_name _itemdata_mesh _itemdata_icon _itemdata_rownumber) (break `/Game/Blueprints/Structures/S_ItemData` (`/Game/Blueprints/Items/BP_ItemBase.ItemData` NewItem)))
  (`/Engine/EditorBlueprintResources/StandardMacros.IsValid` (`self.CurrentItem`)
    (:`Is Valid`
      (return false))
    (:`Is Not Valid`
      (return (`KismetArrayLibrary.Array_Contains` (`self.AllowedInputItems`) _itemdata_rownumber)))))

(fn `DestroyTile`
  (bind _asbp_gamemode (cast `/Game/Blueprints/Player/BP_Gamemode` (`GameplayStatics.GetGameMode`))
    (:`then`
      (`/Game/Blueprints/Player/BP_Gamemode.LoseGame` _asbp_gamemode))
    (:`CastFailed`
      _))
  (`parent.DestroyTile`))

(fn `HasRequiredItems?`
  (params (ItemToCheck :type Integer) (AmountRequired :type Integer))
  (returns (`HasEnough?` :type Boolean))
  (locals (StockpileQuantity :type Integer))
  (set `local.StockpileQuantity` 0)
  (for _array_element (`self.Items`)
    (if (== (`.RowNumber_12_380DBCD342C663ACC04684A073B76B15` (break `/Game/Blueprints/Structures/S_ItemData` _array_element)) ItemToCheck)
      (`/Engine/EditorBlueprintResources/StandardMacros.IncrementInt` (`local.StockpileQuantity`))))
  (return (<= AmountRequired (`local.StockpileQuantity`))))

(fn `RemoveItems`
  (params (ItemToRemove :type Integer) (AmountToRemove :type Integer))
  (locals (NumberRemoved :type Integer))
  (bind _items (`self.Items`))
  (for (_array_element _array_index) _items
    (if (== (`.RowNumber_12_380DBCD342C663ACC04684A073B76B15` (break `/Game/Blueprints/Structures/S_ItemData` _array_element)) ItemToRemove)
      (`/Engine/EditorBlueprintResources/StandardMacros.IncrementInt` (`local.NumberRemoved`)
        (:`  `
          (`KismetArrayLibrary.Array_Remove` _items _array_index)
          (if (not (< (`local.NumberRemoved`) AmountToRemove))
            (break))))))
  (`/Game/Blueprints/UI/W_HUD.UpdateItems` (`self.Hud Ref`) (`self.Items`))
  (return))

(fn `UserConstructionScript`
  (`parent.UserConstructionScript`))