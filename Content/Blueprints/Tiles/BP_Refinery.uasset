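; Refinery tile that burns fuel to convert an input item into its refined version and pass it to the output tile.
; Allowed inputs are either fuel items, consumed into a small capped reserve, or a single held item.
; Tick updates the fuel text, looks up the refined row in DT_Items, reserves a willing target and moves the converted item, briefly playing fire.
; Unrefinable items are destroyed; DoneMoving completes the handoff.
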(event `self.ReceiveTick`
  (params (DeltaSeconds :type "Float (single-precision)"))
  (bind _currentitem (`self.CurrentItem`))
  (bind _currentitem_2 (`self.CurrentItem`))
  (bind _returnvalue (`SceneComponent.K2_GetComponentLocation` (`self.OutputPos`)))
  (bind (_itemdata_name _itemdata_mesh _itemdata_icon _itemdata_rownumber _itemdata_fabricationtype _itemdata_requirements _itemdata_materialoverride _itemdata_refineditem) (break `/Game/Blueprints/Structures/S_ItemData` (`/Game/Blueprints/Items/BP_ItemBase.ItemData` _currentitem_2)))
  (`TextRenderComponent.K2_SetText` (`self.TextRender`) (`KismetTextLibrary.Conv_StringToText` (`KismetStringLibrary.Concat_StrStr` "Fuel: " (`KismetStringLibrary.Conv_IntToString` (`self.Fuel`)) "/5")))
  (`/Engine/EditorBlueprintResources/StandardMacros.IsValid` _currentitem_2
    (:`Is Valid`
      (if (> _itemdata_refineditem 0)
        (if (> (`self.Fuel`) 0)
          (bind _returnvalue_2 (`|GetDataTableRow` "/Game/Blueprints/Datatables/DT_Items.DT_Items" (`KismetStringLibrary.Conv_StringToName` (`KismetStringLibrary.Conv_IntToString` _itemdata_refineditem)))
            (:`then`
              (bind _tileref (message `/Game/Blueprints/Interfaces/BPI_Tile.GetTile` (`BlueprintMapLibrary.Map_Find` (`/Game/Blueprints/BP_TileManager.TileActors` (`self.TileManagerRef`)) (`/Game/Blueprints/Macros/MacroLibrary.WorldToTilePos` _returnvalue))))
              (bind _output_get (set `self.TargetTile` _tileref))
              (bind _canadd_ (message `/Game/Blueprints/Interfaces/BPI_Tile.CanAddItemToTile` _output_get (`self.CurrentItem`)))
              (if _canadd_
                (`/Game/Blueprints/Items/BP_ItemBase.ConvertItemType` _currentitem _returnvalue_2)
                (`/Game/Blueprints/Items/BP_ItemBase.MoveItem` _currentitem self _tileref (`SceneComponent.K2_GetComponentLocation` (`self.Direction`)) _returnvalue)
                (set `/Game/Blueprints/Tiles/BP_TileBase.IsReserved` true _tileref)
                (set `self.Fuel` (`KismetMathLibrary.Clamp` (- (`self.Fuel`) 1) 0 5))
                (`self.ActivateParticle`)))
            (:`RowNotFound`
              (`/Game/Blueprints/Items/BP_ItemBase.DestroyItem` (`self.CurrentItem`) :!label _label)
              (set `self.CurrentItem` null))))
        (else
          (goto _label))))))

(event `/Game/Blueprints/Interfaces/BPI_Tile.AddItemToTile`
  (params (NewItem :type "/Game/Blueprints/Items/BP_ItemBase Object Reference"))
  (bind (_itemdata_name _itemdata_mesh _itemdata_icon _itemdata_rownumber) (break `/Game/Blueprints/Structures/S_ItemData` (`/Game/Blueprints/Items/BP_ItemBase.ItemData` NewItem)))
  (if (== _itemdata_rownumber 3)
    (set `self.Fuel` (`KismetMathLibrary.Clamp` (+ (`self.Fuel`) 1) 0 5))
    (`/Game/Blueprints/Items/BP_ItemBase.DestroyItem` NewItem)
    (else
      (set `self.CurrentItem` NewItem))))

(event `/Game/Blueprints/Interfaces/BPI_Tile.SpawnItemOnConveyor`
  (params (NewItem :type "/Game/Blueprints/Structures/S_ItemData Structure"))
  (bind _returnvalue (`|SpawnActorFromClass` "/Game/Blueprints/Items/BP_ItemBase.BP_ItemBase_C" (`KismetMathLibrary.MakeTransform` (`SplineComponent.GetLocationAtDistanceAlongSpline` (`self.Spline`) 50.0 "World")) "Undefined" "OverrideRootScale" null null))
  (bind _itemref (message `/Game/Blueprints/Items/BPI_Item.GetItem` _returnvalue))
  (bind _output_get (set `self.CurrentItem` _itemref))
  (`/Game/Blueprints/Items/BP_ItemBase.InitItemStats` _output_get NewItem))

(event `self.ReceiveBeginPlay`
  (`ActorComponent.SetActive` (`self.NS_RefineryFire`) false false))

(event `ActivateParticle`
  (`ActorComponent.SetActive` (`self.NS_RefineryFire`) true false)
  (`KismetSystemLibrary.K2_SetTimerDelegate` (delegate `DeactivateParticle`) 1.75))

(event `DeactivateParticle`
  (`ActorComponent.SetActive` (`self.NS_RefineryFire`) false false))

(fn `CanAddItemToTile`
  (params (NewItem :type "/Game/Blueprints/Items/BP_ItemBase Object Reference"))
  (returns (`CanAdd?` :type Boolean))
  (bind (_itemdata_name _itemdata_mesh _itemdata_icon _itemdata_rownumber) (break `/Game/Blueprints/Structures/S_ItemData` (`/Game/Blueprints/Items/BP_ItemBase.ItemData` NewItem)))
  (if (`KismetArrayLibrary.Array_Contains` (`self.AllowedInputItems`) _itemdata_rownumber)
    (if (== _itemdata_rownumber 3)
      (if (< (`self.Fuel`) 5)
        (return true)
        (else
          (return false)))
      (else
        (`/Engine/EditorBlueprintResources/StandardMacros.IsValid` (`self.CurrentItem`)
          (:`Is Valid`
            (return false))
          (:`Is Not Valid`
            (return true)))))
    (else
      (return false))))

(fn `DoneMoving`
  (`/Game/Blueprints/Interfaces/BPI_Tile.AddItemToTile` (`self.TargetTile`) (`self.CurrentItem`))
  (set `self.CurrentItem` null)
  (set `self.IsReserved` false)
  (return))

(fn `GetTile`
  (returns (TileRef :type "/Game/Blueprints/Tiles/BP_TileBase Object Reference"))
  (return self))

(fn `UserConstructionScript`)