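; BP_TilePreview is a preview tile actor that animates a cube's scale when it appears and when it is removed.
; On BeginPlay the ExpandTile timeline scales the Cube component uniformly from its Lerp track.
; RemovePreviewTile, gated by a DoOnce so it runs only once, plays the ShrinkTile timeline on the same scale and destroys the actor when it finishes.
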(event `self.ReceiveBeginPlay`
  (bind (_direction _lerp) (`Timeline|ExpandTile`)
    (:`Update`
      (`SceneComponent.SetRelativeScale3D` (`self.Cube`) (`KismetMathLibrary.Conv_DoubleToVector` _lerp)))))

(event `RemovePreviewTile`
  (`/Engine/EditorBlueprintResources/StandardMacros.DoOnce` false
    (:`Completed`
      (bind (_direction _lerp) (`Timeline|ShrinkTile`)
        (:`Update`
          (`SceneComponent.SetRelativeScale3D` (`self.Cube`) (`KismetMathLibrary.Conv_DoubleToVector` _lerp)))
        (:`Finished`
          (`self.K2_DestroyActor`))))))

(fn `UserConstructionScript`)