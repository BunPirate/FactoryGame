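; BP_Arm is a grid tile that transfers items from the tile behind it to the tile in front.
; When idle, Tick polls the rear tile, takes its item, frees it and attaches the item to GrabPoint as a timeline swings the pivot half a turn.
; While holding, it polls the front tile, hands the item over once accepted and reverses the timeline, returning to idle when that finishes.
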(event `self.ReceiveTick`
  (params (DeltaSeconds :type "Float (single-precision)"))
  (if (`self.Idle?`)
    (`self.AttemptPickup`)
    (elif (`self.HoldingItem`)
      (`self.AttemptDrop`))))

(event `AttemptPickup`
  (bind _tileref (message `/Game/Blueprints/Interfaces/BPI_Tile.GetTile` (`BlueprintMapLibrary.Map_Find` (`/Game/Blueprints/BP_TileManager.TileActors` (`self.TileManagerRef`)) (`/Game/Blueprints/Macros/MacroLibrary.GetCoordInDirectionInverse` (`self.Coordinate`) (`self.TileDirection`)))))
  (`/Engine/EditorBlueprintResources/StandardMacros.IsValid` _tileref
    (:`Is Valid`
      (bind _currentitem (`/Game/Blueprints/Tiles/BP_TileBase.CurrentItem` _tileref))
      (`/Engine/EditorBlueprintResources/StandardMacros.IsValid` _currentitem
        (:`Is Valid`
          (set `self.CurrentItem` _currentitem)
          (set `/Game/Blueprints/Tiles/BP_TileBase.CurrentItem` null _tileref)
          (set `/Game/Blueprints/Tiles/BP_TileBase.IsReserved` false _tileref)
          (set `self.Idle?` false)
          (set `self.HoldingItem` true)
          (`self.K2_AttachToComponent` (`self.CurrentItem`) (`self.GrabPoint`) "None" "SnapToTarget" "KeepWorld" "KeepRelative" true)
          (bind (_direction _lerptrack) (`Timeline|RotateArm` :!label _label)
            (:`Update`
              (`SceneComponent.K2_SetRelativeRotation` (`self.Pivot`) (`KismetMathLibrary.RLerp` (struct :`Pitch` 1e-06) (struct :`Pitch` 1e-06 :`Yaw` 180.0) _lerptrack) false false))
            (:`Finished`
              (if (not (`self.HoldingItem`))
                (set `self.Idle?` true)))))))))

(event `AttemptDrop`
  (bind _currentitem (`self.CurrentItem`))
  (bind _tileref (message `/Game/Blueprints/Interfaces/BPI_Tile.GetTile` (`BlueprintMapLibrary.Map_Find` (`/Game/Blueprints/BP_TileManager.TileActors` (`self.TileManagerRef`)) (`/Game/Blueprints/Macros/MacroLibrary.GetCoordInDirection` (`self.Coordinate`) (`self.TileDirection`)))))
  (`/Engine/EditorBlueprintResources/StandardMacros.IsValid` _tileref
    (:`Is Valid`
      (bind _canadd_ (`/Game/Blueprints/Interfaces/BPI_Tile.CanAddItemToTile` _tileref))
      (if _canadd_
        (`self.K2_DetachFromActor` (`self.CurrentItem`) "KeepWorld" "KeepWorld" "KeepWorld")
        (`/Game/Blueprints/Items/BP_ItemBase.MoveItem` _currentitem self _tileref)
        (`/Game/Blueprints/Interfaces/BPI_Tile.AddItemToTile` _tileref _currentitem)
        (set `self.HoldingItem` false)
        (set `self.CurrentItem` null)
        (goto _label :!via `Reverse`)))))

(event `PickUpItem`
  (params (Item :type "/Game/Blueprints/Items/BP_ItemBase Object Reference")))

(event `DropItem`)

(fn `UserConstructionScript`
  (`parent.UserConstructionScript`))