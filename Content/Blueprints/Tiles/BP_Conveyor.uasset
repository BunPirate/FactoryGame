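; Conveyor tile that carries one item at a time and passes it to the tile it faces on the TileManager grid.
; Each Tick it asks that neighbor through tile messages whether it accepts the item, then starts the item's move and reserves the target.
; DoneMoving hands the item over and clears this tile, and new items spawn at the spline start.
; Older inventory, overlap-push and neighbor-visibility logic remains unwired.
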(event `self.ReceiveTick`
  (params (DeltaSeconds :type "Float (single-precision)"))
  (`/Engine/EditorBlueprintResources/StandardMacros.IsValid` (`self.CurrentItem`)
    (:`Is Valid`
      (bind _tileref (message `/Game/Blueprints/Interfaces/BPI_Tile.GetTile` (`BlueprintMapLibrary.Map_Find` (`/Game/Blueprints/BP_TileManager.TileActors` (`self.TileManagerRef`)) (`/Game/Blueprints/Macros/MacroLibrary.GetCoordInDirection` (`self.Coordinate`) (`self.TileDirection`)))))
      (set `self.TargetTile` _tileref)
      (bind _canadd_ (message `/Game/Blueprints/Interfaces/BPI_Tile.CanAddItemToTile` _tileref (`self.CurrentItem`)))
      (if _canadd_
        (`/Game/Blueprints/Items/BP_ItemBase.MoveItem` (`self.CurrentItem`) self _tileref (`SplineComponent.GetLocationAtDistanceAlongSpline` (`self.Spline`) 50.0 "World") (`self.K2_GetActorLocation` _tileref))
        (set `/Game/Blueprints/Tiles/BP_TileBase.IsReserved` true _tileref)))))

(event `self.AddItemToTile`
  (params (NewItem :type "/Game/Blueprints/Items/BP_ItemBase Object Reference"))
  (set `self.CurrentItem` NewItem))

(event `self.SpawnItemOnConveyor`
  (params (NewItem :type "/Game/Blueprints/Structures/S_ItemData Structure"))
  (bind _returnvalue (`|SpawnActorFromClass` "/Game/Blueprints/Items/BP_ItemBase.BP_ItemBase_C" (`KismetMathLibrary.MakeTransform` (`SplineComponent.GetLocationAtDistanceAlongSpline` (`self.Spline`) 0.0 "World")) "Undefined" "OverrideRootScale" null null))
  (bind _itemref (message `/Game/Blueprints/Items/BPI_Item.GetItem` _returnvalue))
  (bind _output_get (set `self.CurrentItem` _itemref))
  (`/Game/Blueprints/Items/BP_ItemBase.InitItemStats` _output_get NewItem))

(fn `CanAddItemToTile`
  (params (NewItem :type "/Game/Blueprints/Items/BP_ItemBase Object Reference"))
  (returns (`CanAdd?` :type Boolean))
  (`/Engine/EditorBlueprintResources/StandardMacros.IsValid` (`self.CurrentItem`)
    (:`Is Valid`
      (return false))
    (:`Is Not Valid`
      (if (not (`self.IsReserved`))
        (return true)))))

(fn `DoneMoving`
  (`self.AddItemToTile` (`self.TargetTile`) (`self.CurrentItem`))
  (set `self.CurrentItem` null)
  (set `self.IsReserved` false)
  (return))

(fn `GetTile`
  (returns (TileRef :type "/Game/Blueprints/Tiles/BP_TileBase Object Reference"))
  (return self))

(fn `UserConstructionScript`)