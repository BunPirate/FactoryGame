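; Artillery tile that turns items fed into it into ammo and fires projectiles at nearby pawns.
; When Tick finds a held item, it adds ammo if the type matches, clears it, then finds the closest pawn in range via sphere overlap and eases two cubes' yaw and pitch toward it.
; A looping timer spawns a projectile at the fire point, spending ammo, while a target and ammo exist.
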(event `self.ReceiveTick`
  (params (DeltaSeconds :type "Float (single-precision)"))
  (bind _cube (`self.Cube`))
  (bind _currentitem (`self.CurrentItem`))
  (bind (_itemdata_name _itemdata_mesh _itemdata_icon _itemdata_rownumber) (break `/Game/Blueprints/Structures/S_ItemData` (`/Game/Blueprints/Items/BP_ItemBase.ItemData` _currentitem)))
  (`parent.ReceiveTick` DeltaSeconds)
  (`/Engine/EditorBlueprintResources/StandardMacros.IsValid` _currentitem
    (:`Is Valid`
      (if (== (`self.Required Input Item`) _itemdata_rownumber)
        (set `self.CurrentAmmo` (+ (`self.CurrentAmmo`) 5)))
      (set `self.CurrentItem` null)
      (bind _closestenemyactor (`self.GetClosestEnemy`))
      (bind _output_get (set `self.HasTarget` (`KismetSystemLibrary.IsValid` _closestenemyactor)))
      (if _output_get
        (bind (_returnvalue_roll _returnvalue_pitch _returnvalue_yaw) (`KismetMathLibrary.BreakRotator` (`KismetMathLibrary.RInterpTo` (`SceneComponent.RelativeRotation` _cube) (`KismetMathLibrary.FindRelativeLookAtRotation` (`self.GetTransform`) (`self.K2_GetActorLocation` _closestenemyactor)) DeltaSeconds 5.0)))
        (`SceneComponent.K2_SetRelativeRotation` _cube (`KismetMathLibrary.MakeRotator` 0.0 0.0 _returnvalue_yaw) false false)
        (`SceneComponent.K2_SetRelativeRotation` (`self.Cube1`) (`KismetMathLibrary.MakeRotator` 0.0 _returnvalue_pitch) false false)))))

(event `self.ReceiveBeginPlay`
  (`KismetSystemLibrary.K2_SetTimerDelegate` (delegate `Shoot`) (`self.Firedelay`) true))

(event `Shoot`
  (bind (_returnvalue_location _returnvalue_rotation) (`KismetMathLibrary.BreakTransform` (`SceneComponent.K2_GetComponentToWorld` (`self.FirePoint`))))
  (if (and (`self.HasTarget`) (> (`self.CurrentAmmo`) 0))
    (`|SpawnActorFromClass` "/Game/Blueprints/Projectiles/BP_ProjectileBase.BP_ProjectileBase_C" (`KismetMathLibrary.MakeTransform` _returnvalue_location _returnvalue_rotation) "AlwaysSpawn" "OverrideRootScale" null null)
    (set `self.CurrentAmmo` (- (`self.CurrentAmmo`) 1))))

(event `/Game/Blueprints/Interfaces/BPI_Tile.AddItemToTile`
  (params (NewItem :type "/Game/Blueprints/Items/BP_ItemBase Object Reference"))
  (set `self.CurrentItem` NewItem))

(fn `CanAddItemToTile`
  (params (NewItem :type "/Game/Blueprints/Items/BP_ItemBase Object Reference"))
  (returns (`CanAdd?` :type Boolean))
  (`/Engine/EditorBlueprintResources/StandardMacros.IsValid` (`self.CurrentItem`)
    (:`Is Valid`
      (return false))
    (:`Is Not Valid`
      (if (not (`self.IsReserved`))
        (return true)))))

(fn `GetClosestEnemy`
  (returns (ClosestEnemyActor :type "Actor Object Reference"))
  (locals (ClosestDistance :type "Float (double-precision)" :default 9999999999999.0) (ClosestEnemy :type "Actor Object Reference"))
  (bind _outactors (`KismetSystemLibrary.SphereOverlapActors` (`self.K2_GetActorLocation`) (`self.Range`) (`|MakeArray` "ObjectTypeQuery3" :!type "EObjectTypeQuery Enum")))
  (for _array_element _outactors
    (bind _returnvalue (`KismetMathLibrary.Vector_Distance` (`self.K2_GetActorLocation` _array_element) (`self.K2_GetActorLocation`)))
    (if (< _returnvalue (`local.ClosestDistance`))
      (set `local.ClosestDistance` _returnvalue)
      (set `local.ClosestEnemy` _array_element)))
  (return (`local.ClosestEnemy`)))

(fn `GetTile`
  (returns (TileRef :type "/Game/Blueprints/Tiles/BP_TileBase Object Reference"))
  (return self))

(fn `UserConstructionScript`
  (`parent.UserConstructionScript`))