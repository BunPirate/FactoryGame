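; BP_ItemBase is a base actor for items that slide between tiles.
; MoveItem plays a timeline that lerps the item from the current tile to the target tile, held slightly above them, and destroys it if either tile becomes invalid.
; When the move finishes it notifies the current tile through DoneMovingMessage, and GetItem returns the actor itself.
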(event `MoveItem`
  (params (CurrentTile :type "/Game/Blueprints/Tiles/BP_TileBase Object Reference") (TargetTile :type "/Game/Blueprints/Tiles/BP_TileBase Object Reference"))
  (bind (_direction _lerp) (`Timeline|Lerp` :!via `PlayFromStart`)
    (:`Update`
      (`/Engine/EditorBlueprintResources/StandardMacros.IsValid` CurrentTile
        (:`Is Valid`
          (`/Engine/EditorBlueprintResources/StandardMacros.IsValid` TargetTile
            (:`Is Valid`
              (`self.K2_SetActorLocation` (+ (`KismetMathLibrary.VLerp` (`self.K2_GetActorLocation` CurrentTile) (`self.K2_GetActorLocation` TargetTile) _lerp) (0.0 0.0 25.0))))
            (:`Is Not Valid`
              (`self.K2_DestroyActor`))))
        (:`Is Not Valid`
          (`self.K2_DestroyActor`))))
    (:`Finished`
      (message `/Game/Blueprints/Interfaces/BPI_Tile.DoneMoving` CurrentTile))))

(fn `GetItem`
  (returns (ItemRef :type "/Game/Blueprints/Items/BP_ItemBase Object Reference"))
  (return self))

(fn `UserConstructionScript`)