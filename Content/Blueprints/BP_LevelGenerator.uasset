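; Generates a chunked rock terrain level at BeginPlay from seeded FastNoise.
; Thresholded noise fills the RockPositions tile map, which becomes one procedural mesh section per chunk, with rock tiles as raised vertices.
; ClearArea, also called by ClearStartArea, removes rock in a rectangle and collects the chunks of those tiles and their neighbors.
; Those chunks are rebuilt through a delayed loop and prioritized zero-time gameplay tasks, rather than regenerating the whole level.
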(event `self.ReceiveBeginPlay`
  (`self.SetupNoise`)
  (`self.GenerateRockPointChunks`)
  (`self.GenerateRockChunks`))

(event `ClearStartArea`
  (params (Coordinate :type "/Game/Blueprints/Structures/IntVector2 Structure") (AreaSize :type "/Game/Blueprints/Structures/IntVector2 Structure"))
  (`self.ClearArea` Coordinate AreaSize))

(event `ClearArea`
  (params (Coordinate :type "/Game/Blueprints/Structures/IntVector2 Structure") (AreaSize :type "/Game/Blueprints/Structures/IntVector2 Structure"))
  ;[1 1 1] Clear tiles in a specified area
  (for _index (range (+ AreaSize_X_4_6582DAC54E23558CE2425DA215FE3DE3 1))
    (for _index_2 (range (+ AreaSize_Y_5_2CE97EF04AC43C7EE518E4B20F9E68C5 1))
      (bind _rockdata (`self.RemoveRockPoint` (make `/Game/Blueprints/Structures/IntVector2` (+ Coordinate_X_4_6582DAC54E23558CE2425DA215FE3DE3 _index) (+ Coordinate_Y_5_2CE97EF04AC43C7EE518E4B20F9E68C5 _index_2))))
      (bind (_isrock _coordinate _chunk _chunkindex) (break `/Game/Blueprints/Structures/S_RockData` _rockdata))
      (`KismetArrayLibrary.Array_AddUnique` (`self.ChunksToUpdate`) _chunkindex)
      (bind (_up _down _left _right _tiles) (`self.GetNeighboringTiles` _coordinate))
      (for _array_element _tiles
        (`KismetArrayLibrary.Array_AddUnique` (`self.ChunksToUpdate`) (`.ChunkIndex_11_75AE812D4531CD219843369C6C11C4E9` (break `/Game/Blueprints/Structures/S_RockData` (`BlueprintMapLibrary.Map_Find` (`self.RockPositions`) _array_element)))))))
  (bind (_arrayelement _arrayindex) (`/Game/Blueprints/Macros/MacroLibrary.ForEachLoopWithDelay` (`self.ChunksToUpdate`))
    (:`LoopBody`
      (`GameplayTask_WaitDelay.TaskWaitDelay` (`self.GameplayTasks`) 0.0 (+ (`KismetMathLibrary.Conv_IntToByte` _arrayindex) 192)
        (:`then`
          (`self.UpdateRockMeshChunk` _arrayelement))))
    (:`Completed`
      (`KismetArrayLibrary.Array_Clear` (`self.ChunksToUpdate`)))))

(fn `CreateRockMeshChunk`
  (params (ChunkCoord :type "/Game/Blueprints/Structures/IntVector2 Structure") (SectionIndex :type Integer))
  (locals (X :type Integer) (Y :type Integer) (Vertices :type "Array of Vector Structure") (Triangles :type "Array of Integer") (Normals :type "Array of Vector Structure") (Tangents :type "Array of ProcMeshTangent Structure"))
  (bind (_x _y) (break `/Game/Blueprints/Structures/IntVector2` ChunkCoord))
  (bind (_x_2 _y_2) (break `/Game/Blueprints/Structures/IntVector2` ChunkCoord))
  (bind (_chunksize_x _chunksize_y) (break `/Game/Blueprints/Structures/IntVector2` (`self.ChunkSize`)))
  (bind (_chunksize_x_2 _chunksize_y_2) (break `/Game/Blueprints/Structures/IntVector2` (`self.ChunkSize`)))
  (bind (_chunkcoord_x _chunkcoord_y) (break `/Game/Blueprints/Structures/IntVector2` (`local.ChunkCoord`)))
  (bind _tilesize (`self.TileSize`))
  (bind _rockscale (`self.RockScale`))
  (bind (_chunksize_x_3 _chunksize_y_3) (break `/Game/Blueprints/Structures/IntVector2` (`self.ChunkSize`)))
  (bind _intvector2 (make `/Game/Blueprints/Structures/IntVector2` (+ (`local.X`) (* _x _chunksize_x_3)) (+ (* _y _chunksize_y_3) (`local.Y`))))
  (bind _value (`BlueprintMapLibrary.Map_Find` (`self.RockPositions`) _intvector2))
  (bind (_isrock _coordinate _chunk _chunkindex _resourcetype _resourcevalue) (break `/Game/Blueprints/Structures/S_RockData` _value))
  (for _index (range (+ _chunksize_x 1))
    (set `local.X` _index)
    (for _index_2 (range (+ _chunksize_y 1))
      (set `local.Y` _index_2)
      (`BlueprintMapLibrary.Map_Add` (`self.TileChunkIndices`) (make `/Game/Blueprints/Structures/IntVector2` (+ _chunkcoord_x (`local.X`)) (+ _chunkcoord_y (`local.Y`))) (`local.SectionIndex`))
      (`KismetArrayLibrary.Array_Add` (`local.Vertices`) (`KismetMathLibrary.MakeVector` (* (`KismetMathLibrary.Conv_IntToDouble` (+ (* (`local.X`) _rockscale) (* _x_2 _chunksize_x_2))) _tilesize) (* (`KismetMathLibrary.Conv_IntToDouble` (+ (* (`local.Y`) _rockscale) (* _y_2 _chunksize_y_2))) _tilesize) (`KismetMathLibrary.SelectFloat` 250.0 0.0 (`.IsRock_19_5BFF7CF2469715920896CAB6CAEBA798` (break `/Game/Blueprints/Structures/S_RockData` _value)))))
      (`BlueprintMapLibrary.Map_Add` (`self.RockPositions`) _intvector2 (make `/Game/Blueprints/Structures/S_RockData` _isrock _coordinate _chunk (`local.SectionIndex`) _resourcetype _resourcevalue))))
  (bind _triangles (`KismetProceduralMeshLibrary.CreateGridMeshTriangles` (+ (`local.X`) 1) (+ (`local.Y`) 1)))
  (set `local.Triangles` _triangles)
  (bind (_normals _tangents) (`KismetProceduralMeshLibrary.CalculateTangentsForMesh` (`local.Vertices`) (`local.Triangles`)))
  (set `local.Normals` _normals)
  (set `local.Tangents` _tangents)
  (`ProceduralMeshComponent.CreateMeshSection_LinearColor` :`self` (`self.RockProceduralMesh`) :`SectionIndex` SectionIndex :`Vertices` (`local.Vertices`) :`Triangles` (`local.Triangles`) :`Normals` (`local.Normals`) :`Tangents` (`local.Tangents`))
  (`PrimitiveComponent.SetMaterial` (`self.RockProceduralMesh`) SectionIndex "/Game/Materials/M_Rock_Inst.M_Rock_Inst"))

(fn `GenerateRockChunks`
  (locals (ChunkIndex :type Integer))
  (bind (_numofchunks_x _numofchunks_y) (break `/Game/Blueprints/Structures/IntVector2` (`self.NumOfChunks`)))
  (for _index (range (+ _numofchunks_x 1))
    (for _index_2 (range (+ _numofchunks_y 1))
      (`/Engine/EditorBlueprintResources/StandardMacros.IncrementInt` (`local.ChunkIndex`)
        (:`  `
          (`BlueprintMapLibrary.Map_Add` (`self.ChunkCoordinates`) (`local.ChunkIndex`) (make `/Game/Blueprints/Structures/IntVector2` _index _index_2))
          (`self.CreateRockMeshChunk` (make `/Game/Blueprints/Structures/IntVector2` _index _index_2) (`local.ChunkIndex`)))))))

(fn `GenerateRockPointChunks`
  (bind (_numofchunks_x _numofchunks_y) (break `/Game/Blueprints/Structures/IntVector2` (`self.NumOfChunks`)))
  (for _index (range (+ _numofchunks_x 1))
    (for _index_2 (range (+ _numofchunks_y 1))
      (`self.GenerateRockPointsChunk` (make `/Game/Blueprints/Structures/IntVector2` _index _index_2)))))

(fn `GenerateRockPointsChunk`
  (params (ChunkCoordinate :type "/Game/Blueprints/Structures/IntVector2 Structure") (ChunkIndex :type Integer))
  (locals (X :type Integer) (Y :type Integer))
  (bind (_x _y) (break `/Game/Blueprints/Structures/IntVector2` ChunkCoordinate))
  (bind (_x_2 _y_2) (break `/Game/Blueprints/Structures/IntVector2` ChunkCoordinate))
  (bind (_chunksize_x _chunksize_y) (break `/Game/Blueprints/Structures/IntVector2` (`self.ChunkSize`)))
  (bind (_chunksize_x_2 _chunksize_y_2) (break `/Game/Blueprints/Structures/IntVector2` (`self.ChunkSize`)))
  (bind (_chunksize_x_3 _chunksize_y_3) (break `/Game/Blueprints/Structures/IntVector2` (`self.ChunkSize`)))
  (bind _intvector2 (make `/Game/Blueprints/Structures/IntVector2` (+ (* _x_2 _chunksize_x_2) (`local.X`)) (+ (* _y_2 _chunksize_y_2) (`local.Y`))))
  (for _index (range (+ _chunksize_x 1))
    (set `local.X` _index)
    (for _index_2 (range (+ _chunksize_y 1))
      (set `local.Y` _index_2)
      (`BlueprintMapLibrary.Map_Add` (`self.RockPositions`) _intvector2 (make `/Game/Blueprints/Structures/S_RockData` (> (`FastNoiseWrapper.GetNoise2D` (`self.FastNoiseWrapper`) (* (`KismetMathLibrary.Conv_IntToDouble` (+ (`local.X`) (* _x _chunksize_x_3))) 5.0) (* (`KismetMathLibrary.Conv_IntToDouble` (+ (`local.Y`) (* _y _chunksize_y_3))) 5.0)) (`self.NoiseThreshold`)) _intvector2 ChunkCoordinate ChunkIndex)))))

(fn `GetNeighboringTiles`
  (params (Position :type "/Game/Blueprints/Structures/IntVector2 Structure"))
  (returns (Up :type "/Game/Blueprints/Structures/IntVector2 Structure") (Down :type "/Game/Blueprints/Structures/IntVector2 Structure") (Left :type "/Game/Blueprints/Structures/IntVector2 Structure") (Right :type "/Game/Blueprints/Structures/IntVector2 Structure") (Tiles :type "Array of /Game/Blueprints/Structures/IntVector2 Structure"))
  (bind (_x _y) (break `/Game/Blueprints/Structures/IntVector2` Position))
  (bind (_x_2 _y_2) (break `/Game/Blueprints/Structures/IntVector2` Position))
  (bind (_x_3 _y_3) (break `/Game/Blueprints/Structures/IntVector2` Position))
  (bind (_x_4 _y_4) (break `/Game/Blueprints/Structures/IntVector2` Position))
  (bind _intvector2 (make `/Game/Blueprints/Structures/IntVector2` _x (+ _y -1)))
  (bind _intvector2_2 (make `/Game/Blueprints/Structures/IntVector2` (+ _x_2 1) _y_2))
  (bind _intvector2_3 (make `/Game/Blueprints/Structures/IntVector2` (+ _x_3 -1) _y_3))
  (bind _intvector2_4 (make `/Game/Blueprints/Structures/IntVector2` _x_4 (+ _y_4 1)))
  (return _intvector2_4 _intvector2 _intvector2_3 _intvector2_2 (`|MakeArray` _intvector2_4 _intvector2 _intvector2_3 _intvector2_2)))

(fn `RemoveRockPoint`
  (params (Position :type "/Game/Blueprints/Structures/IntVector2 Structure"))
  (returns (RockData :type "/Game/Blueprints/Structures/S_RockData Structure"))
  (locals (ChunksAffected :type "Array of Integer"))
  (bind _rockpositions (`self.RockPositions`))
  (bind (_value _returnvalue) (`BlueprintMapLibrary.Map_Find` _rockpositions Position))
  (bind (_isrock _coordinate _chunk _chunkindex _resourcetype _resourcevalue) (break `/Game/Blueprints/Structures/S_RockData` _value))
  (bind _s_rockdata (make `/Game/Blueprints/Structures/S_RockData` false _coordinate _chunk _chunkindex _resourcetype _resourcevalue))
  (`BlueprintMapLibrary.Map_Add` _rockpositions Position _s_rockdata)
  (if _returnvalue
    (return _s_rockdata)))

(fn `SetupNoise`
  (bind _returnvalue (`|GenericCreateObject` self "/Script/FastNoiseGenerator.FastNoiseWrapper"))
  (bind _output_get (set `self.FastNoiseWrapper` _returnvalue))
  (`FastNoiseWrapper.SetupFastNoise` _output_get "Simplex" (`self.Seed`) 0.01 "Quintic" "FBM" 3 2.0 0.5 0.45 "Euclidean" "CellValue")
  (return))

(fn `UpdateRockMeshChunk`
  (params (SectionIndex :type Integer))
  (locals (X :type Integer) (Y :type Integer) (Vertices :type "Array of Vector Structure") (Triangles :type "Array of Integer") (Normals :type "Array of Vector Structure") (Tangents :type "Array of ProcMeshTangent Structure"))
  (bind (_chunksize_x _chunksize_y) (break `/Game/Blueprints/Structures/IntVector2` (`self.ChunkSize`)))
  (bind _tilesize (`self.TileSize`))
  (bind (_chunksize_x_2 _chunksize_y_2) (break `/Game/Blueprints/Structures/IntVector2` (`self.ChunkSize`)))
  (bind _rockscale (`self.RockScale`))
  (bind (_chunksize_x_3 _chunksize_y_3) (break `/Game/Blueprints/Structures/IntVector2` (`self.ChunkSize`)))
  (bind _value (`BlueprintMapLibrary.Map_Find` (`self.ChunkCoordinates`) SectionIndex))
  (bind (_x _y) (break `/Game/Blueprints/Structures/IntVector2` _value))
  (bind (_x_2 _y_2) (break `/Game/Blueprints/Structures/IntVector2` _value))
  (bind (_x_3 _y_3) (break `/Game/Blueprints/Structures/IntVector2` _value))
  (bind (_vertices _triangles _normals _uvs _tangents) (`KismetProceduralMeshLibrary.GetSectionFromProceduralMesh` (`self.RockProceduralMesh`) SectionIndex))
  (`|ExecutionSequence`
    (:`then_0`
      (set `local.Triangles` _triangles))
    (:`then_1`
      (set `local.Normals` _normals))
    (:`then_2`
      (set `local.Tangents` _tangents))
    (:`then_3`
      (`KismetArrayLibrary.Array_Clear` (`local.Vertices`))
      (for _index (range (+ _chunksize_x 1))
        (set `local.X` _index)
        (for _index_2 (range (+ _chunksize_y 1))
          (set `local.Y` _index_2)
          (`BlueprintMapLibrary.Map_Add` (`self.TileChunkIndices`) (make `/Game/Blueprints/Structures/IntVector2` (+ _x_2 (`local.X`)) (+ _y_2 (`local.Y`))) (`local.SectionIndex`))
          (`KismetArrayLibrary.Array_Add` (`local.Vertices`) (`KismetMathLibrary.MakeVector` (* (`KismetMathLibrary.Conv_IntToDouble` (+ (* (`local.X`) _rockscale) (* _x _chunksize_x_2))) _tilesize) (* (`KismetMathLibrary.Conv_IntToDouble` (+ (* (`local.Y`) _rockscale) (* _y _chunksize_y_2))) _tilesize) (`KismetMathLibrary.SelectFloat` 250.0 0.0 (`.IsRock_19_5BFF7CF2469715920896CAB6CAEBA798` (break `/Game/Blueprints/Structures/S_RockData` (`BlueprintMapLibrary.Map_Find` (`self.RockPositions`) (make `/Game/Blueprints/Structures/IntVector2` (+ (`local.X`) (* _x_3 _chunksize_x_3)) (+ (* _y_3 _chunksize_y_3) (`local.Y`)))))))))))
      (bind _triangles_2 (`KismetProceduralMeshLibrary.CreateGridMeshTriangles` (+ (`local.X`) 1) (+ (`local.Y`) 1)))
      (set `local.Triangles` _triangles_2)
      (bind (_normals_2 _tangents_2) (`KismetProceduralMeshLibrary.CalculateTangentsForMesh` (`local.Vertices`) (`local.Triangles`)))
      (set `local.Normals` _normals_2)
      (set `local.Tangents` _tangents_2)
      (`ProceduralMeshComponent.UpdateMeshSection_LinearColor` :`self` (`self.RockProceduralMesh`) :`SectionIndex` SectionIndex :`Vertices` (`local.Vertices`) :`Normals` (`local.Normals`) :`Tangents` (`local.Tangents`)))))

(fn `UpdateRockMeshPoint`
  (params (Position :type "/Game/Blueprints/Structures/IntVector2 Structure"))
  (locals (X :type Integer) (Y :type Integer) (Vertices :type "Array of Vector Structure") (Triangles :type "Array of Integer") (Normals :type "Array of Vector Structure") (Tangents :type "Array of ProcMeshTangent Structure"))
  (bind (_chunksize_x _chunksize_y) (break `/Game/Blueprints/Structures/IntVector2` (`self.ChunkSize`)))
  (bind _tilesize (`self.TileSize`))
  (bind _x (`local.X`))
  (bind _y (`local.Y`))
  (bind (_isrock _coordinate _chunk _chunkindex) (break `/Game/Blueprints/Structures/S_RockData` (`BlueprintMapLibrary.Map_Find` (`self.RockPositions`) (make `/Game/Blueprints/Structures/IntVector2` _x _y))))
  (for _index (range (+ _chunksize_x 1))
    (set `local.X` _index)
    (for _index_2 (range (+ _chunksize_y 1))
      (set `local.Y` _index_2)
      (`KismetArrayLibrary.Array_Add` (`local.Vertices`) (`KismetMathLibrary.MakeVector` (* (`KismetMathLibrary.Conv_IntToDouble` _x) _tilesize) (* (`KismetMathLibrary.Conv_IntToDouble` _y) _tilesize) (`KismetMathLibrary.SelectFloat` 250.0 0.0 _isrock)))))
  (bind _triangles (`KismetProceduralMeshLibrary.CreateGridMeshTriangles` (+ (`local.X`) 1) (+ (`local.Y`) 1)))
  (set `local.Triangles` _triangles)
  (bind (_normals _tangents) (`KismetProceduralMeshLibrary.CalculateTangentsForMesh` (`local.Vertices`) (`local.Triangles`)))
  (set `local.Normals` _normals)
  (set `local.Tangents` _tangents)
  (`ProceduralMeshComponent.UpdateMeshSection_LinearColor` :`self` (`self.RockProceduralMesh`) :`SectionIndex` _chunkindex :`Vertices` (`local.Vertices`) :`Normals` (`local.Normals`) :`Tangents` (`local.Tangents`)))

(fn `UserConstructionScript`)