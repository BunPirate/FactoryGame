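; BP_TileManager manages the building grid, spawns the Core near the level center, and spawns wave-tiered enemies toward the level edges.
; Placement checks occupancy and ground type from BP_LevelGenerator, then pays costs from the Core, which serves as stockpile.
; Multi-tile footprints rotate by Direction through axis swaps and sign flips, mapping every covered coordinate to one actor in TileActors.
; Player demolition refunds costs unless the building is protected.
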(event `self.ReceiveBeginPlay`
  (bind _returnvalue (`GameplayStatics.GetActorOfClass` "/Game/Blueprints/BP_LevelGenerator.BP_LevelGenerator_C"))
  (set `self.LevelGeneratorRef` _returnvalue)
  (`self.SpawnCore`))

(event `SpawnCore`
  (bind _levelgeneratorref (`self.LevelGeneratorRef`))
  (bind (_numofchunks_x _numofchunks_y) (break `/Game/Blueprints/Structures/IntVector2` (`/Game/Blueprints/BP_LevelGenerator.NumOfChunks` _levelgeneratorref)))
  (bind (_chunksize_x _chunksize_y) (break `/Game/Blueprints/Structures/IntVector2` (`/Game/Blueprints/BP_LevelGenerator.ChunkSize` _levelgeneratorref)))
  (bind _returnvalue (* _numofchunks_x _chunksize_x))
  (bind _returnvalue_2 (* _numofchunks_y _chunksize_y))
  (set `self.LevelSize` (make `/Game/Blueprints/Structures/IntVector2` _returnvalue _returnvalue_2))
  (bind _output_get (set `self.CenterCoord` (make `/Game/Blueprints/Structures/IntVector2` (/ _returnvalue 2) (/ _returnvalue_2 2))))
  (bind _returnvalue_3 (`|GetDataTableRow` "/Game/Blueprints/Datatables/DT_BuildingData.DT_BuildingData" "1")
    (:`then`
      (bind (_x _y) (break `/Game/Blueprints/Structures/IntVector2` _output_get))
      (bind _intvector2 (make `/Game/Blueprints/Structures/IntVector2` (+ _x (`KismetMathLibrary.RandomIntegerInRange` -10 10)) (+ _y (`KismetMathLibrary.RandomIntegerInRange` -10 10))))
      (bind _isvalidarea (`self.CheckTilesInArea` _intvector2 (`.Size_15_4B26410D4E4F8DF384A9C0AB67D49E38` (break `/Game/Blueprints/Structures/S_BuildingInfo` _returnvalue_3)) :!label _label))
      (if _isvalidarea
        (bind (_success_ _buildingref) (`self.PlaceMultiTileBuilding` _intvector2 "NewEnumerator0" _returnvalue_3))
        (if _success_
          (bind _asbp_core (cast `/Game/Blueprints/Tiles/BP_Core` _buildingref))
          (set `self.StockpileRef` _asbp_core)
          (else
            (goto _label)))
        (else
          (goto _label))))))

(fn `CheckTile`
  (params (Coordinate :type "/Game/Blueprints/Structures/IntVector2 Structure"))
  (returns (`IsEmpty?` :type Boolean))
  (bind (_value _returnvalue) (`BlueprintMapLibrary.Map_Find` (`/Game/Blueprints/BP_LevelGenerator.RockPositions` (`self.LevelGeneratorRef`)) Coordinate))
  ;[1 1 1] Has a rock in position
  (if _returnvalue
    (if (`|EnumEquality` (`.GroundType_21_5BFF7CF2469715920896CAB6CAEBA798` (break `/Game/Blueprints/Structures/S_RockData` _value)) "NewEnumerator0")
      _
      (else
        (return false))))
  ;[1 1 1] Has a tile in pos
  (if (`.ReturnValue` (`BlueprintMapLibrary.Map_Find` (`self.TileActors`) Coordinate))
    (return false)
    (else
      (return true))))

(fn `CheckTilesInArea`
  (params (Corner :type "/Game/Blueprints/Structures/IntVector2 Structure (by ref)") (Size :type "/Game/Blueprints/Structures/IntVector2 Structure") (Direction :type "/Game/Blueprints/Enums/E_Direction Enum" :default "NewEnumerator0"))
  (returns (IsValidArea :type Boolean))
  (locals (`ValidArea?` :type Boolean :default true))
  (bind (_x _y) (break `/Game/Blueprints/Structures/IntVector2` Size))
  (bind (_x_2 _y_2) (break `/Game/Blueprints/Structures/IntVector2` Corner))
  ;[1 1 1] X
  (for _index (range _x)
    ;[1 1 1] Y
    (for _index_2 (range _y)
      (bind _returnvalue (* _index (select `/Game/Blueprints/Enums/E_Direction` Direction :`NewEnumerator0` 1 :`NewEnumerator1` -1 :`NewEnumerator2` -1 :`NewEnumerator3` 1)))
      (bind _returnvalue_2 (* _index_2 (select `/Game/Blueprints/Enums/E_Direction` Direction :`NewEnumerator0` 1 :`NewEnumerator1` -1 :`NewEnumerator2` 1 :`NewEnumerator3` -1)))
      (bind _intvector2 (make `/Game/Blueprints/Structures/IntVector2` (+ _x_2 (select `/Game/Blueprints/Enums/E_Direction` Direction :`NewEnumerator0` _returnvalue :`NewEnumerator1` _returnvalue :`NewEnumerator2` _returnvalue_2 :`NewEnumerator3` _returnvalue_2)) (+ _y_2 (select `/Game/Blueprints/Enums/E_Direction` Direction :`NewEnumerator0` _returnvalue_2 :`NewEnumerator1` _returnvalue_2 :`NewEnumerator2` _returnvalue :`NewEnumerator3` _returnvalue))))
      (if (`.ReturnValue` (`BlueprintMapLibrary.Map_Find` (`self.TileActors`) _intvector2))
        (set `local.ValidArea?` false)
        (elif (not (`|EnumEquality` (break `/Game/Blueprints/Structures/S_RockData` (`BlueprintMapLibrary.Map_Find` (`/Game/Blueprints/BP_LevelGenerator.RockPositions` (`self.LevelGeneratorRef`)) _intvector2)) "NewEnumerator0"))
          (set `local.ValidArea?` false)))))
  (return (`local.ValidArea?`)))

(fn `NewEnemy`
  (params (Coordinate :type "/Game/Blueprints/Structures/IntVector2 Structure") (EnemyTypes :type "Array of Actor Class Reference (by ref)"))
  (bind (_x _y) (break `/Game/Blueprints/Structures/IntVector2` Coordinate))
  (bind _tilesize (`self.TileSize`))
  (`|SpawnActorFromClass` (`KismetArrayLibrary.Array_Random` EnemyTypes) (`KismetMathLibrary.MakeTransform` (`KismetMathLibrary.MakeVector` (* (`KismetMathLibrary.Conv_IntToDouble` _x) _tilesize) (* (`KismetMathLibrary.Conv_IntToDouble` _y) _tilesize) 250.0)) "AlwaysSpawn" "OverrideRootScale" null null)
  (return))

(fn `Place Tile`
  (params (Coordinate :type "/Game/Blueprints/Structures/IntVector2 Structure") (BuildingData :type "/Game/Blueprints/Structures/S_BuildingInfo Structure") (Direction :type "/Game/Blueprints/Enums/E_Direction Enum" :default "NewEnumerator0"))
  (locals (HasEnoughItems :type Boolean :default true))
  (bind (_name _icon _class _size _multitile _notplayerdestroyable _requireditemsandquantities) (break `/Game/Blueprints/Structures/S_BuildingInfo` BuildingData))
  (bind _coordinate (`local.Coordinate`))
  (bind _stockpileref (`self.StockpileRef`))
  (bind _isempty_ (`self.CheckTile` Coordinate))
  (if _isempty_
    ;[1 1 1] Check if stockpile has enough resources
    (bind _keys (`BlueprintMapLibrary.Map_Keys` _requireditemsandquantities))
    (for (_array_element _array_index) _keys
      (bind _values (`BlueprintMapLibrary.Map_Values` _requireditemsandquantities))
      (`/Engine/EditorBlueprintResources/StandardMacros.IsValid` _stockpileref
        (:`Is Valid`
          (bind _hasenough_ (`/Game/Blueprints/Tiles/BP_Core.HasRequiredItems?` _stockpileref _array_element (`|GetArrayItem` _values _array_index)))
          (if (not _hasenough_)
            (set `local.HasEnoughItems` false)))))
    (if (`local.HasEnoughItems`)
      (`/Engine/EditorBlueprintResources/StandardMacros.IsValid` _stockpileref
        (:`Is Valid`
          (for (_array_element_2 _array_index_2) _keys
            (bind _values_2 (`BlueprintMapLibrary.Map_Values` _requireditemsandquantities))
            (`/Game/Blueprints/Tiles/BP_Core.RemoveItems` _stockpileref _array_element_2 (`|GetArrayItem` _values_2 _array_index_2))))
        (:`Is Not Valid`
          _))
      (bind _returnvalue (`|SpawnActorFromClass` (`.Class_12_248DEC514AD03388FC3266BBC7A5AB6F` (break `/Game/Blueprints/Structures/S_BuildingInfo` BuildingData)) (`KismetMathLibrary.MakeTransform` (`/Game/Blueprints/Macros/MacroLibrary.TileToWorldPos` Coordinate (`self.TileSize`)) (`KismetMathLibrary.MakeRotator` 0.0 0.0 (select `/Game/Blueprints/Enums/E_Direction` Direction :`NewEnumerator1` 180.0 :`NewEnumerator2` -90.0 :`NewEnumerator3` 90.0 :!type "Float (single-precision)"))) "AlwaysSpawn" "OverrideRootScale" null null))
      (message `/Game/Blueprints/Interfaces/BPI_Tile.InitializeTile` _returnvalue self (`self.LevelGeneratorRef`) _coordinate Direction BuildingData (`|MakeArray` _coordinate))
      (`BlueprintMapLibrary.Map_Add` (`self.TileActors`) (`local.Coordinate`) _returnvalue)
      (return)
      (else
        (return)))
    (else
      (return))))

(fn `PlaceMultiTileBuilding`
  (params (Coordinate :type "/Game/Blueprints/Structures/IntVector2 Structure") (Direction :type "/Game/Blueprints/Enums/E_Direction Enum" :default "NewEnumerator0") (BuildingData :type "/Game/Blueprints/Structures/S_BuildingInfo Structure"))
  (returns (`Success?` :type Boolean) (BuildingRef :type "/Game/Blueprints/Tiles/BP_TileBase Object Reference"))
  (locals (NewBuildingCoords :type "Array of /Game/Blueprints/Structures/IntVector2 Structure") (HasEnoughItems :type Boolean :default true))
  (bind (_name _icon _class _size _multitile _notplayerdestroyable _requireditemsandquantities) (break `/Game/Blueprints/Structures/S_BuildingInfo` BuildingData))
  (bind (_x _y) (break `/Game/Blueprints/Structures/IntVector2` Coordinate))
  (bind (_name_2 _icon_2 _class_2 _size_2) (break `/Game/Blueprints/Structures/S_BuildingInfo` BuildingData))
  (bind _stockpileref (`self.StockpileRef`))
  (bind (_x_2 _y_2) (break `/Game/Blueprints/Structures/IntVector2` (`.Size_15_4B26410D4E4F8DF384A9C0AB67D49E38` (break `/Game/Blueprints/Structures/S_BuildingInfo` BuildingData))))
  (bind _isvalidarea (`self.CheckTilesInArea` Coordinate _size_2 Direction))
  (if _isvalidarea
    ;[1 1 1] Check if stockpile has enough resources
    (bind _keys (`BlueprintMapLibrary.Map_Keys` _requireditemsandquantities))
    (for (_array_element _array_index) _keys
      (bind _values (`BlueprintMapLibrary.Map_Values` _requireditemsandquantities))
      (`/Engine/EditorBlueprintResources/StandardMacros.IsValid` _stockpileref
        (:`Is Valid`
          (bind _hasenough_ (`/Game/Blueprints/Tiles/BP_Core.HasRequiredItems?` _stockpileref _array_element (`|GetArrayItem` _values _array_index)))
          (if (not _hasenough_)
            (set `local.HasEnoughItems` false)))))
    (if (`local.HasEnoughItems`)
      (`/Engine/EditorBlueprintResources/StandardMacros.IsValid` _stockpileref
        (:`Is Valid`
          (for (_array_element_2 _array_index_2) _keys
            (bind _values_2 (`BlueprintMapLibrary.Map_Values` _requireditemsandquantities))
            (`/Game/Blueprints/Tiles/BP_Core.RemoveItems` _stockpileref _array_element_2 (`|GetArrayItem` _values_2 _array_index_2))))
        (:`Is Not Valid`
          _))
      (bind _returnvalue (`|SpawnActorFromClass` _class_2 (`KismetMathLibrary.MakeTransform` (`/Game/Blueprints/Macros/MacroLibrary.TileToWorldPos` Coordinate (`self.TileSize`)) (`KismetMathLibrary.MakeRotator` 0.0 0.0 (select `/Game/Blueprints/Enums/E_Direction` Direction :`NewEnumerator1` 180.0 :`NewEnumerator2` -90.0 :`NewEnumerator3` 90.0 :!type "Float (single-precision)"))) "AlwaysSpawn" "OverrideRootScale" null null))
      ;[1 1 1] X
      (for _index (range _x_2)
        ;[1 1 1] Y
        (for _index_2 (range _y_2)
          (bind _returnvalue_2 (* _index (select `/Game/Blueprints/Enums/E_Direction` Direction :`NewEnumerator0` 1 :`NewEnumerator1` -1 :`NewEnumerator2` -1 :`NewEnumerator3` 1)))
          (bind _returnvalue_3 (* _index_2 (select `/Game/Blueprints/Enums/E_Direction` Direction :`NewEnumerator0` 1 :`NewEnumerator1` -1 :`NewEnumerator2` 1 :`NewEnumerator3` -1)))
          (bind _intvector2 (make `/Game/Blueprints/Structures/IntVector2` (+ _x (select `/Game/Blueprints/Enums/E_Direction` Direction :`NewEnumerator0` _returnvalue_2 :`NewEnumerator1` _returnvalue_2 :`NewEnumerator2` _returnvalue_3 :`NewEnumerator3` _returnvalue_3)) (+ _y (select `/Game/Blueprints/Enums/E_Direction` Direction :`NewEnumerator0` _returnvalue_3 :`NewEnumerator1` _returnvalue_3 :`NewEnumerator2` _returnvalue_2 :`NewEnumerator3` _returnvalue_2))))
          (`BlueprintMapLibrary.Map_Add` (`self.TileActors`) _intvector2 _returnvalue)
          (`KismetArrayLibrary.Array_Add` (`local.NewBuildingCoords`) _intvector2)))
      (message `/Game/Blueprints/Interfaces/BPI_Tile.InitializeTile` _returnvalue self (`self.LevelGeneratorRef`) (`local.Coordinate`) Direction BuildingData (`local.NewBuildingCoords`))
      (return true _returnvalue)
      (else
        (return false null)))
    (else
      (return false null))))

(fn `RemoveBuilding`
  (params (Coordinate :type "/Game/Blueprints/Structures/IntVector2 Structure") (`PlayerDestroyed?` :type Boolean))
  (bind _stockpileref (`self.StockpileRef`))
  (bind (_value _returnvalue) (`BlueprintMapLibrary.Map_Find` (`self.TileActors`) Coordinate))
  (if _returnvalue
    (bind _tileref (message `/Game/Blueprints/Interfaces/BPI_Tile.GetTile` _value))
    (`/Engine/EditorBlueprintResources/StandardMacros.IsValid` _tileref
      (:`Is Valid`
        (if `PlayerDestroyed?`
          (bind (_buildingdata_name _buildingdata_icon _buildingdata_class _buildingdata_size _buildingdata_multitile _buildingdata_notplayerdestroyable _buildingdata_requireditemsandquantities) (break `/Game/Blueprints/Structures/S_BuildingInfo` (`/Game/Blueprints/Tiles/BP_TileBase.BuildingData` _tileref)))
          (if (not _buildingdata_notplayerdestroyable)
            (bind _keys (`BlueprintMapLibrary.Map_Keys` _buildingdata_requireditemsandquantities))
            (for (_array_element _array_index) _keys
              (bind _values (`BlueprintMapLibrary.Map_Values` _buildingdata_requireditemsandquantities))
              (`/Game/Blueprints/Tiles/BP_Core.AddManyItems` _stockpileref _array_element (`|GetArrayItem` _values _array_index))
              (`/Game/Blueprints/UI/W_HUD.UpdateItems` (`/Game/Blueprints/Tiles/BP_Core.Hud Ref` _stockpileref) (`/Game/Blueprints/Tiles/BP_Core.Items` _stockpileref)))
            (`/Game/Blueprints/Tiles/BP_TileBase.DestroyTile` _tileref))
          (else
            (`/Game/Blueprints/Tiles/BP_TileBase.DestroyTile` _tileref)))))))

(fn `SpawnEnemies`
  (params (NumberOfEnemies :type Integer) (Wave :type Integer))
  (bind _enemytypes3 (`self.EnemyTypes3`))
  (bind (_levelsize_x _levelsize_y) (break `/Game/Blueprints/Structures/IntVector2` (`self.LevelSize`)))
  (bind _returnvalue (/ _levelsize_y 4))
  (bind _returnvalue_2 (/ _levelsize_x 4))
  (for _ (range NumberOfEnemies)
    ;[1 1 1] Checks if the coordinate is a valid spawn location, if not, find new location
    (bind _output_get (set `self.RandomCoord` (make `/Game/Blueprints/Structures/IntVector2` (`KismetMathLibrary.SelectInt` (`KismetMathLibrary.RandomIntegerInRange` 0 _returnvalue_2) (`KismetMathLibrary.RandomIntegerInRange` (* _returnvalue_2 3) _levelsize_x) (`KismetMathLibrary.RandomBoolWithWeight` 0.5)) (`KismetMathLibrary.SelectInt` (`KismetMathLibrary.RandomIntegerInRange` 0 _returnvalue) (`KismetMathLibrary.RandomIntegerInRange` (* _returnvalue 3) _levelsize_y) (`KismetMathLibrary.RandomBoolWithWeight` 0.5))) :!label _label))
    (bind _isempty_ (`self.CheckTile` _output_get))
    (if _isempty_
      (`self.NewEnemy` (`self.RandomCoord`) (select `bool` (>= Wave 5) :`false` (`self.EnemyTypes1`) :`true` (select `bool` (>= Wave 15) :`false` (`self.EnemyTypes2`) :`true` (select `bool` (>= Wave 25) :`false` _enemytypes3 :`true` _enemytypes3))))
      (else
        (goto _label))))
  (return))

(fn `UserConstructionScript`)